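; Bookshelf actor that slides its mesh along its relative X axis when the MoveBookshelf event is called.
; The event runs once through a DoOnce, storing the mesh's current relative location and a target offset along X.
; A timeline then lerps between the two and feeds only the X component into the mesh's relative location.
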(event `MoveBookshelf`
  (bind _relativelocation (`SceneComponent.RelativeLocation` (`self.SM_Bookshelf_SM_Bookshelf`)))
  (`/Engine/EditorBlueprintResources/StandardMacros.DoOnce` false
    (:`Completed`
      (set `self.InitialLocation` _relativelocation)
      (set `self.TargetLocation` (`KismetMathLibrary.MakeVector` (- (.x _relativelocation) -125.0)))
      (bind (_direction _newtrack_0) (`Timeline|BookshelfMove` :!via `PlayFromStart`)
        (:`Update`
          (bind _returnvalue_x (`KismetMathLibrary.BreakVector` (`KismetMathLibrary.VLerp` (`self.InitialLocation`) (`self.TargetLocation`) _newtrack_0)))
          (`SceneComponent.K2_SetRelativeLocation` (`self.SM_Bookshelf_SM_Bookshelf`) (`KismetMathLibrary.MakeVector` _returnvalue_x) false false))))))

(fn `UserConstructionScript`)