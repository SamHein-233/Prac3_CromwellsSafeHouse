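; BP_Sink is an interactable sink where the player uses a held drain magnet to retrieve a key.
; A box overlap shows the interact prompt; interacting with the magnet removes both and positions the magnet above the sink.
; Two timelines lerp the magnet down and, after a delay, the key up.
; Both actors are then destroyed, the has-key flag is set, a key-added widget shows briefly and the hint advances.
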(event `self.ReceiveBeginPlay`)

(event `self.Box.OnComponentBeginOverlap`
  (params (OverlappedComponent :type "PrimitiveComponent Object Reference") (OtherActor :type "Actor Object Reference") (OtherComp :type "PrimitiveComponent Object Reference") (OtherBodyIndex :type Integer) (bFromSweep :type Boolean) (SweepResult :type "HitResult Structure (by ref)"))
  (cast `/Game/FirstPerson/Blueprints/BP_FirstPersonCharacter` OtherActor)
  (bind _returnvalue (`|CreateWidget` "/Game/Widgets/W_EInteract.W_EInteract_C"))
  (bind _output_get (set `self.InteractWidget_Ref` _returnvalue))
  (`UserWidget.AddToViewport` _output_get 0))

(event `self.Box.OnComponentEndOverlap`
  (params (OverlappedComponent :type "PrimitiveComponent Object Reference") (OtherActor :type "Actor Object Reference") (OtherComp :type "PrimitiveComponent Object Reference") (OtherBodyIndex :type Integer))
  (`WidgetLayoutLibrary.RemoveAllWidgets`))

(event `/Game/Blueprints/Interactables/BPI_Interactable.InteractWith`
  (params (PlayerChar :type "/Game/FirstPerson/Blueprints/BP_FirstPersonCharacter Object Reference"))
  (bind _hints (`self.Hints`))
  (bind _playerref (`self.PlayerRef`))
  (bind (_magnet_initiallocation_x _magnet_initiallocation_y) (`KismetMathLibrary.BreakVector` (`self.Magnet_InitialLocation`)))
  (bind (_returnvalue_location _returnvalue_rotation _returnvalue_scale) (`KismetMathLibrary.BreakTransform` (`SceneComponent.K2_GetComponentToWorld` (`self.DefaultSceneRoot`))))
  (bind _relativelocation (`SceneComponent.RelativeLocation` (`Actor.RootComponent` (`self.MagnetRef`))))
  (bind _output_get (set `self.PlayerRef` PlayerChar))
  (if (`KismetMathLibrary.ClassIsChildOf` (`GameplayStatics.GetObjectClass` (`/Game/FirstPerson/Blueprints/BP_FirstPersonCharacter.HeldItem` _output_get)) "/Game/Blueprints/Sink/BP_DrainMagnet.BP_DrainMagnet_C")
    (`Widget.RemoveFromParent` (`self.InteractWidget_Ref`))
    (`ActorComponent.K2_DestroyComponent` (`self.Box`))
    (bind _output_get_2 (set `self.MagnetRef` (`/Game/FirstPerson/Blueprints/BP_FirstPersonCharacter.HeldItem` _playerref)))
    (`self.K2_DetachFromActor` _output_get_2 "KeepWorld" "KeepWorld" "KeepWorld")
    (set `/Game/FirstPerson/Blueprints/BP_FirstPersonCharacter.HeldItem` null _playerref)
    (`SceneComponent.K2_SetWorldTransform` (`Actor.RootComponent` (`self.MagnetRef`)) (`KismetMathLibrary.MakeTransform` (+ _returnvalue_location (0.0 -30.0 130.0)) (struct :`Roll` 180.0) _returnvalue_scale) false false)
    (set `self.Magnet_InitialLocation` _relativelocation)
    (set `self.Magnet_TargetLocation` (`KismetMathLibrary.MakeVector` 0.0 0.0 (- (.z _relativelocation) 70.0)))
    (`KismetSystemLibrary.Delay` 1.0)
    (`self.KeyGoesUp`)
    (bind (_direction _newtrack_0) (`Timeline|MagnetGoesIntoDrain` :!via `PlayFromStart`)
      (:`Update`
        (bind (_returnvalue_x _returnvalue_y _returnvalue_z) (`KismetMathLibrary.BreakVector` (`KismetMathLibrary.VLerp` (`self.Magnet_InitialLocation`) (`self.Magnet_TargetLocation`) _newtrack_0)))
        (`SceneComponent.K2_SetWorldLocation` (`/Game/Blueprints/Interactables/Items/BP_ItemParent.StaticMesh` (`self.MagnetRef`)) (`KismetMathLibrary.MakeVector` _magnet_initiallocation_x _magnet_initiallocation_y _returnvalue_z) false false))
      (:`Finished`
        (`PrimitiveComponent.SetCollisionEnabled` (`/Game/Blueprints/Interactables/Items/BP_ItemParent.StaticMesh` (`self.MagnetRef`)) "QueryOnly")
        (`KismetSystemLibrary.Delay` 2.0)
        (`self.K2_DestroyActor` (`self.MagnetRef`))
        (`self.K2_DestroyActor` (`self.KeyRef`))
        (set `self.PlayHasKey?` true)
        (cast `/Game/FirstPerson/Blueprints/BP_FirstPersonCharacter` (stale `self.Box.OnComponentBeginOverlap` OtherActor))
        (bind _returnvalue (`|CreateWidget` "/Game/Widgets/W_KeyAdded.W_KeyAdded_C"))
        (bind _output_get_3 (set `self.KeyWidget_Ref` _returnvalue))
        (`UserWidget.AddToViewport` _output_get_3 0)
        (`KismetSystemLibrary.Delay` 5.0)
        (`Widget.RemoveFromParent` (`self.KeyWidget_Ref`))
        (set `/Game/Blueprints/BP_HintController.Row Index` 6 _hints)
        (`/Game/Blueprints/BP_HintController.Current Hint` _hints)))))

(event `KeyGoesUp`
  (bind (_key_initiallocation_x _key_initiallocation_y) (`KismetMathLibrary.BreakVector` (`self.Key_InitialLocation`)))
  (`KismetSystemLibrary.Delay` 3.0)
  (bind _returnvalue (`GameplayStatics.GetActorOfClass` "/Game/Blueprints/Sink/BP_Key.BP_Key_C"))
  (bind _output_get (set `self.KeyRef` _returnvalue))
  (bind _relativelocation (`SceneComponent.RelativeLocation` (`Actor.RootComponent` _output_get)))
  (set `self.Key_InitialLocation` _relativelocation)
  (set `self.Key_TargetLocation` (`KismetMathLibrary.MakeVector` 0.0 0.0 (+ (.z _relativelocation) 37.0)))
  (bind (_direction _newtrack_0) (`Timeline|MagnetTakesKey` :!via `PlayFromStart`)
    (:`Update`
      (bind (_returnvalue_x _returnvalue_y _returnvalue_z) (`KismetMathLibrary.BreakVector` (`KismetMathLibrary.VLerp` (`self.Key_InitialLocation`) (`self.Key_TargetLocation`) _newtrack_0)))
      (`SceneComponent.K2_SetWorldLocation` (`/Game/Blueprints/Sink/BP_Key.SM_Key` (`self.KeyRef`)) (`KismetMathLibrary.MakeVector` _key_initiallocation_x _key_initiallocation_y _returnvalue_z) false false))))

(fn `UserConstructionScript`)