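; BP_HintController steps through the hint rows in the DT_Hints data table, playing each hint's 2D audio.
; BeginPlay runs an endless loop that shows the current hint, waits a fixed delay, then increments RowIndex.
; CurrentHint bounds-checks the index against the row names, prints the name and plays that row's Audio.
; CheckStep is an empty stub, and a disconnected column-reading dialogue graph never runs.
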(event `self.ReceiveBeginPlay`
  (`self.Current Hint` :!label _label)
  (`KismetSystemLibrary.Delay` 3.0)
  (`self.Next Hint`)
  (goto _label))

(event `Current Hint`
  (bind _row_index (`self.Row Index`))
  ;[1 1 1] Gets Row Names for the Puzzle Steps
  (bind _outrownames (`DataTableFunctionLibrary.GetDataTableRowNames` "/Game/Blueprints/DT_Hints.DT_Hints"))
  (if (<= _row_index (- (`KismetArrayLibrary.Array_Length` _outrownames) 1))
    (bind _output (`|GetArrayItem` _outrownames _row_index))
    (bind _returnvalue (`|GetDataTableRow` "/Game/Blueprints/DT_Hints.DT_Hints" _output)
      (:`then`
        (bind _returnvalue_2 (`KismetStringLibrary.Conv_NameToString` _output))
        (`KismetSystemLibrary.PrintString` _returnvalue_2 true true (struct :`G` 1.0 :`B` 0.102636 :`A` 1.0) 10.0 "RowYes")
        (`|ExecutionSequence`
          (:`then_0`
            (`GameplayStatics.PlaySound2D` (`.Audio_20_F5E6241F4F74EAC00B4B96A98FCA4A2D` (break `/Game/Blueprints/S_Hints` _returnvalue)) 1.0 1.0 0.0 null null false))))
      (:`RowNotFound`
        (`KismetSystemLibrary.PrintString` _returnvalue_2 true true (struct :`R` 1.0 :`B` 0.011436 :`A` 1.0) 10.0 "RowNo")))))

(event `Next Hint`
  (set `self.Row Index` (+ (`self.Row Index`) 1)))

(event `Check Step`)

(fn `UserConstructionScript`)