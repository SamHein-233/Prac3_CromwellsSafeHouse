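; BP_Ledger is an interactable ledger that the first-person player can view through a dedicated camera.
; Overlapping its box shows a W_VInteract prompt and enables input on the actor; leaving removes the prompt and disables input.
; IA_View swaps the prompt for the W_Viewing widget created at BeginPlay, sets UI-only input, then finds BP_LedgerCam by class and calls GoToCamera.
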(event `self.ReceiveBeginPlay`
  (bind _returnvalue (`|CreateWidget` "/Game/Widgets/W_Viewing.W_Viewing_C"))
  (set `self.ViewingWidg_Ref` _returnvalue))

(event `EnhancedInput|/Game/FirstPerson/Input/Actions/IA_View`
  (params (ActionValue :type Boolean) (ElapsedSeconds :type "Float (double-precision)") (TriggeredSeconds :type "Float (double-precision)") (InputAction :type "InputAction Object Reference" :default "/Game/FirstPerson/Input/Actions/IA_View.IA_View"))
  (:`Triggered`
    (`Widget.RemoveFromParent` (`self.InteractWidg_Ref`))
    (bind _returnvalue (`UserWidget.AddToPlayerScreen` (`self.ViewingWidg_Ref`) 0))
    (`WidgetBlueprintLibrary.SetInputMode_UIOnlyEx` (`Pawn.GetLocalViewingPlayerController` (stale `self.Box.OnComponentBeginOverlap` _asbp_first_person_character)) null "DoNotLock" _returnvalue)
    (bind _returnvalue_2 (`GameplayStatics.GetActorOfClass` "/Game/Blueprints/Ledger/BP_LedgerCam.BP_LedgerCam_C"))
    (bind _output_get (set `self.Cam_Ref` _returnvalue_2))
    (`/Game/Blueprints/Ledger/BP_LedgerCam.GoToCamera` _output_get)))

(event `self.Box.OnComponentBeginOverlap`
  (params (OverlappedComponent :type "PrimitiveComponent Object Reference") (OtherActor :type "Actor Object Reference") (OtherComp :type "PrimitiveComponent Object Reference") (OtherBodyIndex :type Integer) (bFromSweep :type Boolean) (SweepResult :type "HitResult Structure (by ref)"))
  (bind _asbp_first_person_character (cast `/Game/FirstPerson/Blueprints/BP_FirstPersonCharacter` OtherActor))
  (bind _returnvalue (`|CreateWidget` "/Game/Widgets/W_VInteract.W_VInteract_C"))
  (bind _output_get (set `self.InteractWidg_Ref` _returnvalue))
  (`UserWidget.AddToViewport` _output_get 0)
  (`self.EnableInput` (`GameplayStatics.GetPlayerController` 0)))

(event `self.Box.OnComponentEndOverlap`
  (params (OverlappedComponent :type "PrimitiveComponent Object Reference") (OtherActor :type "Actor Object Reference") (OtherComp :type "PrimitiveComponent Object Reference") (OtherBodyIndex :type Integer))
  (`Widget.RemoveFromParent` (`self.InteractWidg_Ref`))
  (cast `/Game/FirstPerson/Blueprints/BP_FirstPersonCharacter` OtherActor)
  (`self.DisableInput` (`GameplayStatics.GetPlayerController` 0)))

(fn `UserConstructionScript`)