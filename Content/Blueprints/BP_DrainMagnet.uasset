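; BP_DrainMagnet is an interactable drain magnet that the first-person character can use when inside its Box trigger.
; Entering the box shows a W_Interact prompt and enables input on the actor; leaving removes all widgets and disables that input.
; IA_Interact removes the prompt, calls an attach on the player character with Cylinder as parent and hand_rSocket as socket, then disables Cylinder collision.
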(event `self.Box.OnComponentBeginOverlap`
  (params (OverlappedComponent :type "PrimitiveComponent Object Reference") (OtherActor :type "Actor Object Reference") (OtherComp :type "PrimitiveComponent Object Reference") (OtherBodyIndex :type Integer) (bFromSweep :type Boolean) (SweepResult :type "HitResult Structure (by ref)"))
  (cast `/Game/FirstPerson/Blueprints/BP_FirstPersonCharacter` OtherActor)
  (bind _returnvalue (`|CreateWidget` "/Game/Widgets/W_Interact.W_Interact_C"))
  (bind _output_get (set `self.InteractWid_Ref` _returnvalue))
  (`UserWidget.AddToViewport` _output_get 0)
  (`self.EnableInput` (`GameplayStatics.GetPlayerController` 0)))

(event `self.Box.OnComponentEndOverlap`
  (params (OverlappedComponent :type "PrimitiveComponent Object Reference") (OtherActor :type "Actor Object Reference") (OtherComp :type "PrimitiveComponent Object Reference") (OtherBodyIndex :type Integer))
  (`WidgetLayoutLibrary.RemoveAllWidgets`)
  (cast `/Game/FirstPerson/Blueprints/BP_FirstPersonCharacter` OtherActor)
  (`self.DisableInput` (`GameplayStatics.GetPlayerController` 0)))

(event `EnhancedInput|/Game/FirstPerson/Input/Actions/IA_Interact`
  (params (ActionValue :type Boolean) (ElapsedSeconds :type "Float (double-precision)") (TriggeredSeconds :type "Float (double-precision)") (InputAction :type "InputAction Object Reference" :default "/Game/FirstPerson/Input/Actions/IA_Interact.IA_Interact"))
  (bind _cylinder (`self.Cylinder`))
  (:`Triggered`
    (`Widget.RemoveFromParent` (`self.InteractWid_Ref`))
    (`self.K2_AttachToComponent` (`GameplayStatics.GetPlayerCharacter` 0) _cylinder "hand_rSocket" "KeepRelative" "KeepRelative" "KeepRelative" true)
    (`PrimitiveComponent.SetCollisionEnabled` _cylinder "NoCollision")))

(fn `UserConstructionScript`)