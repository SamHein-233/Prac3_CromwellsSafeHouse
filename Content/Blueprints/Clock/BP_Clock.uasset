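; BP_Clock is an interactable puzzle clock that opens BP_Cabinet when its hands show the correct time.
; A box overlap shows a view prompt and enables input, and IA_View switches to the clock camera and UI.
; Rotate events step both hands with timelines behind DoOnce gates, checking the time as the minute hand finishes.
; On a match, it returns to the player after a delay and opens the cabinet.
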(event `self.ReceiveBeginPlay`
  (bind _returnvalue (`|CreateWidget` "/Game/Widgets/W_Clock.W_Clock_C"))
  (set `self.ClockWidget_Ref` _returnvalue))

(event `self.Box.OnComponentBeginOverlap`
  (params (OverlappedComponent :type "PrimitiveComponent Object Reference") (OtherActor :type "Actor Object Reference") (OtherComp :type "PrimitiveComponent Object Reference") (OtherBodyIndex :type Integer) (bFromSweep :type Boolean) (SweepResult :type "HitResult Structure (by ref)"))
  (bind _asbp_first_person_character (cast `/Game/FirstPerson/Blueprints/BP_FirstPersonCharacter` OtherActor))
  (bind _returnvalue (`|CreateWidget` "/Game/Widgets/W_VInteract.W_VInteract_C"))
  (bind _output_get (set `self.ViewWidget_Ref` _returnvalue))
  (`UserWidget.AddToViewport` _output_get 0)
  (`self.EnableInput` (`GameplayStatics.GetPlayerController` 0)))

(event `EnhancedInput|/Game/FirstPerson/Input/Actions/IA_View`
  (params (ActionValue :type Boolean) (ElapsedSeconds :type "Float (double-precision)") (TriggeredSeconds :type "Float (double-precision)") (InputAction :type "InputAction Object Reference" :default "/Game/FirstPerson/Input/Actions/IA_View.IA_View"))
  (:`Triggered`
    (`Widget.RemoveFromParent` (`self.ViewWidget_Ref`))
    (bind _returnvalue (`UserWidget.AddToPlayerScreen` (`self.ClockWidget_Ref`) 0))
    (`WidgetBlueprintLibrary.SetInputMode_UIOnlyEx` (`Pawn.GetLocalViewingPlayerController` (stale `self.Box.OnComponentBeginOverlap` _asbp_first_person_character)) null "DoNotLock" _returnvalue)
    (bind _returnvalue_2 (`GameplayStatics.GetActorOfClass` "/Game/Blueprints/Clock/BP_ClockCam.BP_ClockCam_C"))
    (bind _output_get (set `self.ClockCam_Ref` _returnvalue_2))
    (`/Game/Blueprints/Clock/BP_ClockCam.GoToCamera` _output_get)))

(event `self.Box.OnComponentEndOverlap`
  (params (OverlappedComponent :type "PrimitiveComponent Object Reference") (OtherActor :type "Actor Object Reference") (OtherComp :type "PrimitiveComponent Object Reference") (OtherBodyIndex :type Integer))
  (`Widget.RemoveFromParent` (`self.ViewWidget_Ref`))
  (cast `/Game/FirstPerson/Blueprints/BP_FirstPersonCharacter` OtherActor)
  (`self.DisableInput` (`GameplayStatics.GetPlayerController` 0)))

(event `RotateHandsRight`
  (bind (_min_currentrotation_roll _min_currentrotation_pitch) (`KismetMathLibrary.BreakRotator` (`self.Min_CurrentRotation`)))
  (bind (_hour_currentrotation_roll _hour_currentrotation_pitch) (`KismetMathLibrary.BreakRotator` (`self.Hour_CurrentRotation`)))
  (`|ExecutionSequence`
    (:`then_0`
      (`/Engine/EditorBlueprintResources/StandardMacros.DoOnce` false :!label _label
        (:`Completed`
          (bind _output_get (set `self.Min_CurrentRotation` (`KismetMathLibrary.MakeRotator` 0.0 (+ _min_currentrotation_pitch -30.0))))
          (set `self.Min_TargetRotation` (`KismetMathLibrary.MakeRotator` 0.0 (.pitch _output_get)))
          (bind (_direction _newtrack_0) (`Timeline|RotateMinHandRight` :!via `PlayFromStart`)
            (:`Update`
              (bind (_returnvalue_roll _returnvalue_pitch) (`KismetMathLibrary.BreakRotator` (`KismetMathLibrary.RLerp` (`self.Min_InitialRotation`) (`self.Min_TargetRotation`) _newtrack_0)))
              (`SceneComponent.K2_SetRelativeRotation` (`self.SM_Clock_SM_MinHand`) (`KismetMathLibrary.MakeRotator` 0.0 _returnvalue_pitch) false false))
            (:`Finished`
              (set `self.Min_InitialRotation` (`self.Min_TargetRotation`))
              (`self.CheckClockTime`)
              (`KismetSystemLibrary.PrintString` (`KismetStringLibrary.Conv_RotatorToString` (`self.Min_CurrentRotation`)))
              (goto _label :!via `Reset`))))))
    (:`then_1`
      (`/Engine/EditorBlueprintResources/StandardMacros.DoOnce` false :!label _label_2
        (:`Completed`
          (bind _output_get_2 (set `self.Hour_CurrentRotation` (`KismetMathLibrary.MakeRotator` 0.0 (+ _hour_currentrotation_pitch -2.5))))
          (bind (_returnvalue_roll_2 _returnvalue_pitch_2) (`KismetMathLibrary.BreakRotator` (`KismetMathLibrary.MakeRotator` 0.0 (.pitch _output_get_2))))
          (set `self.Hour_TargetRotation` (`KismetMathLibrary.MakeRotator` 0.0 _returnvalue_pitch_2))
          (bind (_direction_2 _newtrack_0_2) (`Timeline|RotateHourHandRight` :!via `PlayFromStart`)
            (:`Update`
              (bind (_returnvalue_roll_3 _returnvalue_pitch_3) (`KismetMathLibrary.BreakRotator` (`KismetMathLibrary.RLerp` (`self.Hour_InitialRotation`) (`self.Hour_TargetRotation`) _newtrack_0_2)))
              (`SceneComponent.K2_SetRelativeRotation` (`self.SM_Clock_SM_HourHand`) (`KismetMathLibrary.MakeRotator` 180.0 _returnvalue_pitch_3) false false))
            (:`Finished`
              (set `self.Hour_InitialRotation` (`self.Hour_TargetRotation`))
              (`KismetSystemLibrary.PrintString` (`KismetStringLibrary.Conv_RotatorToString` (`self.Hour_CurrentRotation`)) true true (struct :`R` 0.460012 :`B` 1.0 :`A` 1.0))
              (goto _label_2 :!via `Reset`))))))))

(event `RotateHandsLeft`
  (bind (_min_currentrotation_roll _min_currentrotation_pitch) (`KismetMathLibrary.BreakRotator` (`self.Min_CurrentRotation`)))
  (bind (_hour_currentrotation_roll _hour_currentrotation_pitch) (`KismetMathLibrary.BreakRotator` (`self.Hour_CurrentRotation`)))
  (`|ExecutionSequence`
    (:`then_0`
      (`/Engine/EditorBlueprintResources/StandardMacros.DoOnce` false :!label _label_3
        (:`Completed`
          (bind _output_get (set `self.Min_CurrentRotation` (`KismetMathLibrary.MakeRotator` 0.0 (+ _min_currentrotation_pitch 30.0))))
          (set `self.Min_TargetRotation` (`KismetMathLibrary.MakeRotator` 0.0 (.pitch _output_get)))
          (bind (_direction _newtrack_0) (`Timeline|RotateMinHandLeft` :!via `PlayFromStart`)
            (:`Update`
              (bind (_returnvalue_roll _returnvalue_pitch) (`KismetMathLibrary.BreakRotator` (`KismetMathLibrary.RLerp` (`self.Min_InitialRotation`) (`self.Min_TargetRotation`) _newtrack_0)))
              (`SceneComponent.K2_SetRelativeRotation` (`self.SM_Clock_SM_MinHand`) (`KismetMathLibrary.MakeRotator` 0.0 _returnvalue_pitch) false false))
            (:`Finished`
              (set `self.Min_InitialRotation` (`self.Min_TargetRotation`))
              (`self.CheckClockTime`)
              (goto _label_3 :!via `Reset`))))))
    (:`then_1`
      (`/Engine/EditorBlueprintResources/StandardMacros.DoOnce` false
        (:`Completed`
          (bind _output_get_2 (set `self.Hour_CurrentRotation` (`KismetMathLibrary.MakeRotator` 0.0 (+ _hour_currentrotation_pitch 2.5))))
          (bind (_returnvalue_roll_2 _returnvalue_pitch_2) (`KismetMathLibrary.BreakRotator` (`KismetMathLibrary.MakeRotator` 0.0 (.pitch _output_get_2))))
          (set `self.Hour_TargetRotation` (`KismetMathLibrary.MakeRotator` 0.0 _returnvalue_pitch_2))
          (bind (_direction_2 _newtrack_0_2) (`Timeline|RotateHourHandLeft` :!via `PlayFromStart`)
            (:`Update`
              (bind (_returnvalue_roll_3 _returnvalue_pitch_3) (`KismetMathLibrary.BreakRotator` (`KismetMathLibrary.RLerp` (`self.Hour_InitialRotation`) (`self.Hour_TargetRotation`) _newtrack_0_2)))
              (`SceneComponent.K2_SetRelativeRotation` (`self.SM_Clock_SM_HourHand`) (`KismetMathLibrary.MakeRotator` 180.0 _returnvalue_pitch_3) false false))
            (:`Finished`
              (set `self.Hour_InitialRotation` (`self.Hour_TargetRotation`)))))))))

(event `TimeCorrect`
  (bind _returnvalue (`GameplayStatics.GetPlayerController` 0))
  (`KismetSystemLibrary.Delay` 3.0)
  (`/Game/Blueprints/Clock/BP_ClockCam.GoToPlayer` (`self.ClockCam_Ref`) (`GameplayStatics.GetPlayerCharacter` 0))
  (`WidgetBlueprintLibrary.SetInputMode_GameOnly` _returnvalue)
  (set `PlayerController.bShowMouseCursor` false _returnvalue)
  (`Widget.RemoveFromParent` (`self.ClockWidget_Ref`))
  (bind _returnvalue_2 (`GameplayStatics.GetActorOfClass` "/Game/Blueprints/Lockboxes/Cabinets/BP_Cabinet.BP_Cabinet_C"))
  (`/Game/Blueprints/Lockboxes/Cabinets/BP_Cabinet.OpenDoor` _returnvalue_2))

(fn `CheckClockTime`
  (bind (_min_currentrotation_roll _min_currentrotation_pitch) (`KismetMathLibrary.BreakRotator` (`self.Min_CurrentRotation`)))
  (bind (_hour_currentrotation_roll _hour_currentrotation_pitch) (`KismetMathLibrary.BreakRotator` (`self.Hour_CurrentRotation`)))
  (if (and (== (`self.CorrectMinRotation`) _min_currentrotation_pitch) (== (`self.CorrectHourRotation`) _hour_currentrotation_pitch))
    (`KismetSystemLibrary.PrintString` "Time correct!")
    (`self.TimeCorrect`)
    (else
      (`KismetSystemLibrary.PrintString` "Not correct time"))))

(fn `UserConstructionScript`)