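; BP_Desk is an interactable desk whose drawer, once DrawerUnlocked is true, opens to grant the escape key.
; A trigger box shows the interact widget and enables input for the overlapping first-person character while unlocked.
; Secondary interact runs once, removing the latch, calling MoveEvidence on BP_Evidence and sliding the drawer with a Timeline lerp.
; On finish it removes the box and prompt, sets HasEscapeKey and plays audio cues.
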(event `self.ReceiveBeginPlay`
  (bind _returnvalue (`|CreateWidget` "/Game/Widgets/W_FInteract.W_FInteract_C"))
  (set `self.Wig_Interaction_Ref` _returnvalue)
  (bind _returnvalue_2 (`GameplayStatics.GetActorOfClass` "/Game/Blueprints/Interactables/Items/BP_Evidence.BP_Evidence_C"))
  (set `self.BPEvidence_Ref` _returnvalue_2))

(event `EnhancedInput|/Game/FirstPerson/Input/Actions/IA_SecondaryInteract`
  (params (ActionValue :type Boolean) (ElapsedSeconds :type "Float (double-precision)") (TriggeredSeconds :type "Float (double-precision)") (InputAction :type "InputAction Object Reference" :default "/Game/FirstPerson/Input/Actions/IA_SecondaryInteract.IA_SecondaryInteract"))
  (bind _relativelocation (`SceneComponent.RelativeLocation` (`self.SM_Desk_SM_Drawer`)))
  (:`Triggered`
    (if (`self.DrawerUnlocked?`)
      (`/Engine/EditorBlueprintResources/StandardMacros.DoOnce` false
        (:`Completed`
          (`ActorComponent.K2_DestroyComponent` (`self.SM_Desk_SM_Latch`))
          (`/Game/Blueprints/Interactables/Items/BP_Evidence.MoveEvidence` (`self.BPEvidence_Ref`))
          (set `self.InitialLocation` _relativelocation)
          (set `self.TargetLocation` (`KismetMathLibrary.MakeVector` (- (.x _relativelocation) 32.0)))
          (`GameplayStatics.PlaySound2D` "/Game/Blueprints/Audio/Wooden_Drawer/Drawer_Open.Drawer_Open" 1.0 1.0 0.0 null null)
          (bind (_direction _newtrack_0) (`Timeline|Timeline` :!via `PlayFromStart`)
            (:`Update`
              (bind _returnvalue_x (`KismetMathLibrary.BreakVector` (`KismetMathLibrary.VLerp` (`self.InitialLocation`) (`self.TargetLocation`) _newtrack_0)))
              (`SceneComponent.K2_SetRelativeLocation` (`self.SM_Desk_SM_Drawer`) (`KismetMathLibrary.MakeVector` _returnvalue_x) false false))
            (:`Finished`
              (`ActorComponent.K2_DestroyComponent` (`self.Box`))
              (`Widget.RemoveFromParent` (`self.Wig_Interaction_Ref`))
              (set `self.HasEscapeKey` true)
              (`GameplayStatics.PlaySound2D` "/Game/Blueprints/Audio/Alert_Sounds/MS_Alert.MS_Alert" 1.0 1.0 0.0 null null)
              (`KismetSystemLibrary.Delay` 0.8)
              (`GameplayStatics.PlaySound2D` "/Game/Blueprints/Audio/Dialogue/CromwellDialogue/Puzzle_8_1.Puzzle_8_1" 1.0 1.0 0.0 null null)))))
      (else
        (`KismetSystemLibrary.PrintString` "Drawer Still Locked")))))

(event `self.Box.OnComponentBeginOverlap`
  (params (OverlappedComponent :type "PrimitiveComponent Object Reference") (OtherActor :type "Actor Object Reference") (OtherComp :type "PrimitiveComponent Object Reference") (OtherBodyIndex :type Integer) (bFromSweep :type Boolean) (SweepResult :type "HitResult Structure (by ref)"))
  (cast `/Game/FirstPerson/Blueprints/BP_FirstPersonCharacter` OtherActor)
  (if (`self.DrawerUnlocked?`)
    (`UserWidget.AddToViewport` (`self.Wig_Interaction_Ref`) 0)
    (`self.EnableInput` (`GameplayStatics.GetPlayerController` 0))))

(event `self.Box.OnComponentEndOverlap`
  (params (OverlappedComponent :type "PrimitiveComponent Object Reference") (OtherActor :type "Actor Object Reference") (OtherComp :type "PrimitiveComponent Object Reference") (OtherBodyIndex :type Integer))
  (cast `/Game/FirstPerson/Blueprints/BP_FirstPersonCharacter` OtherActor)
  (`Widget.RemoveFromParent` (`self.Wig_Interaction_Ref`))
  (`self.DisableInput` (`GameplayStatics.GetPlayerController` 0)))

(fn `UserConstructionScript`)