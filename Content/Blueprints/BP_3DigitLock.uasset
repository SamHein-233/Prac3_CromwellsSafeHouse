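; BP_3DigitLock is an interactable three-digit lock that the first-person character operates through a UI widget.
; A box overlap shows an interact prompt and enables input, so E opens the lock widget in UI-only mode and calls GoToCamera on BP_3DigitLockCam.
; Timelines lerp the first dial 35 degrees left or right in yaw.
; The selected row is stored but unused in rotation, and no combination check exists here.
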(event `self.ReceiveBeginPlay`
  (bind _returnvalue (`|CreateWidget` "/Game/Widgets/W_3DigitLock.W_3DigitLock_C"))
  (set `self.DigitWidget_Ref` _returnvalue))

(event `RotateRight`
  (bind _sm_3dial1 (`self.SM_3Dial1`))
  (bind _relativerotation (`SceneComponent.RelativeRotation` _sm_3dial1))
  (bind _output_get (set `self.TargetRelativeRotation` (`KismetMathLibrary.MakeRotator` 0.0 0.0 (`KismetMathLibrary.FClamp` (+ (.yaw _relativerotation) 35.0) -360.0 360.0))))
  (bind (_direction _newtrack_0) (`Timeline|RotateDigit`)
    (:`Update`
      (bind (_returnvalue_roll _returnvalue_pitch _returnvalue_yaw) (`KismetMathLibrary.BreakRotator` (`KismetMathLibrary.RLerp` _relativerotation _output_get _newtrack_0)))
      (`SceneComponent.K2_SetRelativeRotation` _sm_3dial1 (`KismetMathLibrary.MakeRotator` 0.0 0.0 _returnvalue_yaw) false false))))

(event `RotateLeft`
  (bind _sm_3dial1 (`self.SM_3Dial1`))
  (bind _relativerotation (`SceneComponent.RelativeRotation` _sm_3dial1))
  (bind _output_get (set `self.TargetRelativeRotation` (`KismetMathLibrary.MakeRotator` 0.0 0.0 (`KismetMathLibrary.FClamp` (+ (.yaw _relativerotation) -35.0) -360.0 360.0))))
  (bind (_direction _newtrack_0) (`Timeline|Timeline`)
    (:`Update`
      (bind (_returnvalue_roll _returnvalue_pitch _returnvalue_yaw) (`KismetMathLibrary.BreakRotator` (`KismetMathLibrary.RLerp` _relativerotation _output_get _newtrack_0)))
      (`SceneComponent.K2_SetRelativeRotation` _sm_3dial1 (`KismetMathLibrary.MakeRotator` 0.0 0.0 _returnvalue_yaw) false false))))

(event `self.Box.OnComponentBeginOverlap`
  (params (OverlappedComponent :type "PrimitiveComponent Object Reference") (OtherActor :type "Actor Object Reference") (OtherComp :type "PrimitiveComponent Object Reference") (OtherBodyIndex :type Integer) (bFromSweep :type Boolean) (SweepResult :type "HitResult Structure (by ref)"))
  (bind _asbp_first_person_character (cast `/Game/FirstPerson/Blueprints/BP_FirstPersonCharacter` OtherActor))
  (bind _returnvalue (`|CreateWidget` "/Game/Widgets/W_Interact.W_Interact_C"))
  (bind _output_get (set `self.InteractWidget_Ref` _returnvalue))
  (`UserWidget.AddToViewport` _output_get 0)
  (`self.EnableInput` (`GameplayStatics.GetPlayerController` 0)))

(event `Key|E`
  (params (Key :type "Key Structure"))
  (:`Pressed`
    (`Widget.RemoveFromParent` (`self.InteractWidget_Ref`))
    (bind _returnvalue (`UserWidget.AddToPlayerScreen` (`self.DigitWidget_Ref`) 0))
    (`WidgetBlueprintLibrary.SetInputMode_UIOnlyEx` (`Pawn.GetLocalViewingPlayerController` (stale `self.Box.OnComponentBeginOverlap` _asbp_first_person_character)) null "DoNotLock" _returnvalue)
    (bind _returnvalue_2 (`GameplayStatics.GetActorOfClass` "/Game/Blueprints/BP_3DigitLockCam.BP_3DigitLockCam_C"))
    (`/Game/Blueprints/BP_3DigitLockCam.GoToCamera` _returnvalue_2)))

(event `self.Box.OnComponentEndOverlap`
  (params (OverlappedComponent :type "PrimitiveComponent Object Reference") (OtherActor :type "Actor Object Reference") (OtherComp :type "PrimitiveComponent Object Reference") (OtherBodyIndex :type Integer))
  (`WidgetLayoutLibrary.RemoveAllWidgets`)
  (cast `/Game/FirstPerson/Blueprints/BP_FirstPersonCharacter` OtherActor)
  (`self.DisableInput` (`GameplayStatics.GetPlayerController` 0)))

(event `SelectedRow`
  (params (RowIndex :type Integer))
  (set `self.SelectedDigitRow` (`/Game/Widgets/W_3DigitLock.RowIndex` (`self.DigitWidget_Ref`))))

(fn `UserConstructionScript`)