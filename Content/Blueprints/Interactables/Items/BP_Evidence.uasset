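; BP_Evidence is an evidence item actor whose mesh slides aside and then disappears.
; The MoveEvidence event stores the static mesh's relative location and sets a target a short offset along positive local Y.
; A timeline lerps the mesh between the two points without sweeping, then destroys the actor when finished.
; Nothing in this file calls MoveEvidence, and the construction script only runs the parent's.
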(event `MoveEvidence`
  (bind _relativelocation (`SceneComponent.RelativeLocation` (`self.StaticMesh`)))
  (set `self.InitialLocation` _relativelocation)
  (set `self.TargetLocation` (`KismetMathLibrary.MakeVector` (.x _relativelocation) (- (.y _relativelocation) -32.0) (.z _relativelocation)))
  (bind (_direction _newtrack_0) (`Timeline|Timeline` :!via `PlayFromStart`)
    (:`Update`
      (`SceneComponent.K2_SetRelativeLocation` (`self.StaticMesh`) (`KismetMathLibrary.VLerp` (`self.InitialLocation`) (`self.TargetLocation`) _newtrack_0) false false))
    (:`Finished`
      (`self.K2_DestroyActor`))))

(fn `UserConstructionScript`
  (`parent.UserConstructionScript`))