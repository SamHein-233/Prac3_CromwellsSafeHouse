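; BP_Blacklight is a blacklight item whose spot light the player switches on and off.
; The IA_SecondaryInteract input action checks the LightOn flag, then sets the SpotLight intensity to zero or full and flips the flag.
; BeginPlay and the construction script add no logic of their own, and a disconnected copy of the switch-off step never runs.
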(event `self.ReceiveBeginPlay`)

(event `EnhancedInput|/Game/FirstPerson/Input/Actions/IA_SecondaryInteract`
  (params (ActionValue :type Boolean) (ElapsedSeconds :type "Float (double-precision)") (TriggeredSeconds :type "Float (double-precision)") (InputAction :type "InputAction Object Reference" :default "/Game/FirstPerson/Input/Actions/IA_SecondaryInteract.IA_SecondaryInteract"))
  (:`Triggered`
    (if (`self.LightOn?`)
      (`LightComponent.SetIntensity` (`self.SpotLight`) 0.0)
      (set `self.LightOn?` false)
      (else
        (`LightComponent.SetIntensity` (`self.SpotLight`) 5000.0)
        (set `self.LightOn?` true)))))

(fn `UserConstructionScript`
  (`parent.UserConstructionScript`))