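; Base interactable item that the player can pick up, inspect and drop.
; Interacting attaches it to the player's ItemGrip, or inspects it if an item is already held.
; Inspection moves input from player to item for mouse-drag rotation and wheel zoom along the camera's forward vector until IA_Interact ends it.
; Dropping detaches it, places it via a camera line trace and restores physics and collision.
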(event `EnhancedInput|/Game/FirstPerson/Input/Actions/IA_Interact`
  (params (ActionValue :type Boolean) (ElapsedSeconds :type "Float (double-precision)") (TriggeredSeconds :type "Float (double-precision)") (InputAction :type "InputAction Object Reference" :default "/Game/FirstPerson/Input/Actions/IA_Interact.IA_Interact"))
  (:`Started`
    (`self.StopInspect`)))

(event `InputAxisKey|MouseX`
  (params (AxisValue :type "Float (single-precision)"))
  (if (`self.IsRotating?`)
    (`self.K2_SetActorRotation` (`KismetMathLibrary.ComposeRotators` (`self.K2_GetActorRotation`) (`KismetMathLibrary.MakeRotator` 0.0 0.0 (* AxisValue -5.0))))))

(event `/Game/Blueprints/Interactables/BPI_Interactable.InteractWith`
  (params (PlayerChar :type "/Game/FirstPerson/Blueprints/BP_FirstPersonCharacter Object Reference"))
  (bind _output_get (set `self.PlayerRef` PlayerChar))
  (`/Engine/EditorBlueprintResources/StandardMacros.IsValid` (`/Game/FirstPerson/Blueprints/BP_FirstPersonCharacter.HeldItem` _output_get)
    (:`Is Valid`
      (`self.Inspect`))
    (:`Is Not Valid`
      (`self.PickUp`))))

(event `/Game/Blueprints/Interactables/BPI_Interactable.LookAt`
  (params (PlayerChar :type "/Game/FirstPerson/Blueprints/BP_FirstPersonCharacter Object Reference")))

(event `InputAxisKey|MouseY`
  (params (AxisValue :type "Float (single-precision)"))
  (if (`self.IsRotating?`)
    (`self.K2_SetActorRotation` (`KismetMathLibrary.ComposeRotators` (`self.K2_GetActorRotation`) (`KismetMathLibrary.MakeRotator` 0.0 (* AxisValue -5.0))))))

(event `Key|MouseScrollUp`
  (params (Key :type "Key Structure"))
  (bind _returnvalue (`GameplayStatics.GetPlayerCameraManager` 0))
  (:`Pressed`
    (bind _output_get (set `self.ZoomLevel` (`KismetMathLibrary.Clamp` (+ (`self.ZoomLevel`) 1) 1 25)))
    (if (< _output_get 25)
      (`self.K2_SetActorLocation` (+ (`PlayerCameraManager.GetCameraLocation` _returnvalue) (* (`KismetMathLibrary.GetForwardVector` (`PlayerCameraManager.GetCameraRotation` _returnvalue)) (* (`self.ZoomLevel`) 20.0)))))))

(event `Key|LeftMouseButton`
  (params (Key :type "Key Structure"))
  (:`Pressed`
    (set `self.IsRotating?` true))
  (:`Released`
    (set `self.IsRotating?` false)))

(event `Key|MouseScrollDown`
  (params (Key :type "Key Structure"))
  (bind _returnvalue (`GameplayStatics.GetPlayerCameraManager` 0))
  (:`Pressed`
    (bind _output_get (set `self.ZoomLevel` (`KismetMathLibrary.Clamp` (- (`self.ZoomLevel`) 1) 1 20)))
    (if (> _output_get 1)
      (`self.K2_SetActorLocation` (+ (`PlayerCameraManager.GetCameraLocation` _returnvalue) (* (`KismetMathLibrary.GetForwardVector` (`PlayerCameraManager.GetCameraRotation` _returnvalue)) (* (`self.ZoomLevel`) 20.0)))))))

(fn `DropItem`
  (bind _returnvalue (`GameplayStatics.GetPlayerCameraManager` 0))
  (bind _staticmesh (`self.StaticMesh`))
  (bind _returnvalue_2 (`PlayerCameraManager.GetCameraLocation` _returnvalue))
  (`self.K2_DetachFromActor` "KeepWorld" "KeepWorld" "KeepWorld")
  (bind _outhit (`KismetSystemLibrary.LineTraceSingle` :`Start` _returnvalue_2 :`End` (+ _returnvalue_2 (* (`KismetMathLibrary.GetForwardVector` (`PlayerCameraManager.GetCameraRotation` _returnvalue)) 200.0)) :`TraceChannel` "TraceTypeQuery1" :`DrawDebugType` "ForDuration"))
  (bind (_bblockinghit _binitialoverlap _time _distance _location _impactpoint _normal _impactnormal _physmat _hitactor _hitcomponent _hitbonename _bonename _hititem _elementindex _faceindex _tracestart _traceend) (`GameplayStatics.BreakHitResult` _outhit))
  (`self.K2_SetActorLocation` (`KismetMathLibrary.SelectVector` (- _location (* (`self.GetActorForwardVector` (`GameplayStatics.GetPlayerCharacter` 0)) 10.0)) _traceend _bblockinghit))
  (`PrimitiveComponent.SetSimulatePhysics` _staticmesh true)
  (`PrimitiveComponent.SetCollisionEnabled` _staticmesh "QueryAndPhysics")
  (`KismetSystemLibrary.PrintString` (`|GetEnumeratorNameAsString` (`PrimitiveComponent.GetCollisionEnabled` (`self.StaticMesh`)))))

(fn `Inspect`
  (bind _returnvalue (`GameplayStatics.GetPlayerController` 0))
  (bind _returnvalue_2 (`GameplayStatics.GetPlayerCameraManager` 0))
  (`self.DisableInput` (`self.PlayerRef`) _returnvalue)
  (`self.EnableInput` _returnvalue)
  (`self.K2_SetActorLocation` (+ (`PlayerCameraManager.GetCameraLocation` _returnvalue_2) (* (`KismetMathLibrary.GetForwardVector` (`PlayerCameraManager.GetCameraRotation` _returnvalue_2)) 200.0))))

(fn `PickUp`
  (bind _staticmesh (`self.StaticMesh`))
  (`self.K2_AttachToComponent` (`/Game/FirstPerson/Blueprints/BP_FirstPersonCharacter.ItemGrip` (`self.PlayerRef`)) "None" "SnapToTarget" "KeepWorld" "KeepWorld")
  (`PrimitiveComponent.SetSimulatePhysics` _staticmesh false)
  (`PrimitiveComponent.SetCollisionEnabled` _staticmesh "NoCollision")
  (set `/Game/FirstPerson/Blueprints/BP_FirstPersonCharacter.HeldItem` self (`self.PlayerRef`)))

(fn `StopInspect`
  (bind _returnvalue (`GameplayStatics.GetPlayerController` 0))
  (`self.DisableInput` _returnvalue)
  (`self.EnableInput` (`self.PlayerRef`) _returnvalue)
  (`self.K2_SetActorRelativeLocation` (0.0 0.0 0.0)))

(fn `UserConstructionScript`)