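; Lockbox interactable whose lid swings open when a Lookat event fires and the box is unlocked.
; If unlocked, a DoOnce computes a target roll offset from the lid's current rotation and starts a timeline.
; A second DoOnce inside the timeline update applies the lerped roll only on the first update, so the lid does not animate continuously.
; If still locked, it just prints a debug message.
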(event `self.ReceiveBeginPlay`)

(event `self.ReceiveTick`
  (params (DeltaSeconds :type "Float (single-precision)")))

(event `/Game/Blueprints/Interactables/BPI_Interactable.LookAt`
  (params (PlayerChar :type "/Game/FirstPerson/Blueprints/BP_FirstPersonCharacter Object Reference"))
  (bind _relativerotation (`SceneComponent.RelativeRotation` (`self.SM_LockBox_SM_BoxLid`)))
  (if (`self.LockboxUnlocked?`)
    (`/Engine/EditorBlueprintResources/StandardMacros.DoOnce` false
      (:`Completed`
        (bind _output_get (set `self.TargetRotation` (`KismetMathLibrary.MakeRotator` (+ (.roll _relativerotation) -66.0))))
        (bind (_direction _newtrack_0) (`Timeline|Timeline` :!via `PlayFromStart`)
          (:`Update`
            (`/Engine/EditorBlueprintResources/StandardMacros.DoOnce` false
              (:`Completed`
                (bind _returnvalue_roll (`KismetMathLibrary.BreakRotator` (`KismetMathLibrary.RLerp` _output_get _relativerotation _newtrack_0)))
                (`SceneComponent.K2_SetRelativeRotation` (`self.SM_LockBox_SM_BoxLid`) (`KismetMathLibrary.MakeRotator` _returnvalue_roll) false false)))))))
    (else
      (`KismetSystemLibrary.PrintString` "Lock still engaged"))))

(fn `UserConstructionScript`
  (`parent.UserConstructionScript`))