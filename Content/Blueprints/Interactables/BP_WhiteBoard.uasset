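; BP_WhiteBoard is an interactable whiteboard that lets the player pin a held BP_Paper item where they are looking.
; On interact, it detaches the paper, attaches it to the board and places it at a short camera line trace hit, nudged along world -Y.
; It then stands the mesh upright via relative rotation, disables physics, sets query-only collision and clears the player's HeldItem.
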(event `/Game/Blueprints/Interactables/BPI_Interactable.InteractWith`
  (params (PlayerChar :type "/Game/FirstPerson/Blueprints/BP_FirstPersonCharacter Object Reference"))
  (bind _returnvalue (`GameplayStatics.GetPlayerCameraManager` 0))
  (bind _returnvalue_2 (`PlayerCameraManager.GetCameraLocation` _returnvalue))
  (bind _helditem (`/Game/FirstPerson/Blueprints/BP_FirstPersonCharacter.HeldItem` (`self.PlayerRef`)))
  (bind _staticmesh (`/Game/Blueprints/Interactables/Items/BP_ItemParent.StaticMesh` (`/Game/FirstPerson/Blueprints/BP_FirstPersonCharacter.HeldItem` (`self.PlayerRef`))))
  (bind _staticmesh_2 (`/Game/Blueprints/Interactables/Items/BP_ItemParent.StaticMesh` _helditem))
  (bind (_relativerotation_roll _relativerotation_pitch) (`KismetMathLibrary.BreakRotator` (`SceneComponent.RelativeRotation` _staticmesh_2)))
  (bind _output_get (set `self.PlayerRef` PlayerChar))
  (if (`KismetMathLibrary.ClassIsChildOf` (`GameplayStatics.GetObjectClass` (`/Game/FirstPerson/Blueprints/BP_FirstPersonCharacter.HeldItem` _output_get)) "/Game/Blueprints/Interactables/Items/Papers/BP_Paper.BP_Paper_C")
    (`self.K2_DetachFromActor` (`/Game/FirstPerson/Blueprints/BP_FirstPersonCharacter.HeldItem` (`self.PlayerRef`)) "KeepWorld" "KeepWorld" "KeepWorld")
    (bind _outhit (`KismetSystemLibrary.LineTraceSingle` :`Start` _returnvalue_2 :`End` (+ _returnvalue_2 (* (`KismetMathLibrary.GetForwardVector` (`PlayerCameraManager.GetCameraRotation` _returnvalue)) 300.0)) :`TraceChannel` "TraceTypeQuery1" :`bIgnoreSelf` false))
    (`self.K2_AttachToActor` _helditem self "None" "SnapToTarget" "KeepWorld" "KeepWorld" false)
    (`self.K2_SetActorLocation` _helditem (+ (`.Location` (`GameplayStatics.BreakHitResult` _outhit)) (0.0 -1.0 0.0)) false false)
    (`SceneComponent.K2_SetRelativeRotation` _staticmesh_2 (`KismetMathLibrary.MakeRotator` 90.0 _relativerotation_pitch) false false)
    (`PrimitiveComponent.SetSimulatePhysics` _staticmesh false)
    (`PrimitiveComponent.SetCollisionEnabled` _staticmesh "QueryOnly")
    (set `/Game/FirstPerson/Blueprints/BP_FirstPersonCharacter.HeldItem` null (`self.PlayerRef`))))

(fn `UserConstructionScript`)