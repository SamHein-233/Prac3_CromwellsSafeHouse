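; BP_Book is an interactable book that accepts a loose paper item from the player and reveals its page.
; On interaction, a held BP_BookPaper (or subclass) is destroyed, then after a short delay the Page component becomes visible and the player's held item is cleared.
; Otherwise, the book calls Inspect if the player holds another item, or PickUp if their hands are empty.
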(event `/Game/Blueprints/Interactables/BPI_Interactable.InteractWith`
  (params (PlayerChar :type "/Game/FirstPerson/Blueprints/BP_FirstPersonCharacter Object Reference"))
  (bind _helditem (`/Game/FirstPerson/Blueprints/BP_FirstPersonCharacter.HeldItem` (`self.PlayerRef`)))
  (bind _output_get (set `self.PlayerRef` PlayerChar))
  (if (`KismetMathLibrary.ClassIsChildOf` (`GameplayStatics.GetObjectClass` (`/Game/FirstPerson/Blueprints/BP_FirstPersonCharacter.HeldItem` _output_get)) "/Game/Blueprints/Interactables/Items/BP_BookPaper.BP_BookPaper_C")
    (`self.K2_DestroyActor` _helditem)
    (`KismetSystemLibrary.Delay` 0.2)
    (`SceneComponent.SetVisibility` (`self.Page`) true false)
    (set `/Game/FirstPerson/Blueprints/BP_FirstPersonCharacter.HeldItem` null (`self.PlayerRef`))
    (else
      (`/Engine/EditorBlueprintResources/StandardMacros.IsValid` _helditem
        (:`Is Valid`
          (`self.Inspect`))
        (:`Is Not Valid`
          (`self.PickUp`))))))

(fn `UserConstructionScript`)