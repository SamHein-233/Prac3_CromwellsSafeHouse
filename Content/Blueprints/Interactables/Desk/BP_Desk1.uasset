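; Interactable desk whose drawer slides open once when the player uses secondary interact while it is unlocked.
; Overlap of the Box trigger by the first-person character enables input on the desk, with no matching disable.
; Interacting checks DrawerUnlocked, which is not set here, and prints a message if locked.
; Otherwise it destroys the latch, slides the drawer along local X with a Timeline-driven lerp, then destroys the trigger.
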(event `EnhancedInput|/Game/FirstPerson/Input/Actions/IA_SecondaryInteract`
  (params (ActionValue :type Boolean) (ElapsedSeconds :type "Float (double-precision)") (TriggeredSeconds :type "Float (double-precision)") (InputAction :type "InputAction Object Reference" :default "/Game/FirstPerson/Input/Actions/IA_SecondaryInteract.IA_SecondaryInteract"))
  (bind _relativelocation (`SceneComponent.RelativeLocation` (`self.SM_Desk_SM_Drawer`)))
  (:`Triggered`
    (if (`self.DrawerUnlocked?`)
      (`/Engine/EditorBlueprintResources/StandardMacros.DoOnce` false
        (:`Completed`
          (`ActorComponent.K2_DestroyComponent` (`self.SM_Desk_SM_Latch`))
          (set `self.InitialLocation` _relativelocation)
          (set `self.TargetLocation` (`KismetMathLibrary.MakeVector` (- (.x _relativelocation) 32.0)))
          (bind (_direction _newtrack_0) (`Timeline|Timeline` :!via `PlayFromStart`)
            (:`Update`
              (bind _returnvalue_x (`KismetMathLibrary.BreakVector` (`KismetMathLibrary.VLerp` (`self.InitialLocation`) (`self.TargetLocation`) _newtrack_0)))
              (`SceneComponent.K2_SetRelativeLocation` (`self.SM_Desk_SM_Drawer`) (`KismetMathLibrary.MakeVector` _returnvalue_x) false false))
            (:`Finished`
              (`ActorComponent.K2_DestroyComponent` (`self.Box`))))))
      (else
        (`KismetSystemLibrary.PrintString` "Drawer Still Locked")))))

(event `self.Box.OnComponentBeginOverlap`
  (params (OverlappedComponent :type "PrimitiveComponent Object Reference") (OtherActor :type "Actor Object Reference") (OtherComp :type "PrimitiveComponent Object Reference") (OtherBodyIndex :type Integer) (bFromSweep :type Boolean) (SweepResult :type "HitResult Structure (by ref)"))
  (cast `/Game/FirstPerson/Blueprints/BP_FirstPersonCharacter` OtherActor)
  (`self.EnableInput` (`GameplayStatics.GetPlayerController` 0)))

(fn `UserConstructionScript`)