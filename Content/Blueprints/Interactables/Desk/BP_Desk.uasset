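; BP_Desk is an interactable desk whose drawer slides open when the player uses the Interact input.
; A box overlap with the first-person character shows an interact widget and enables input on the desk; leaving clears all widgets and disables input.
; Interacting removes the prompt and plays a timeline that lerps the drawer's relative X to an offset from its current position, with no closing or already-open check.
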(event `EnhancedInput|/Game/FirstPerson/Input/Actions/IA_Interact`
  (params (ActionValue :type Boolean) (ElapsedSeconds :type "Float (double-precision)") (TriggeredSeconds :type "Float (double-precision)") (InputAction :type "InputAction Object Reference" :default "/Game/FirstPerson/Input/Actions/IA_Interact.IA_Interact"))
  (bind _relativelocation (`SceneComponent.RelativeLocation` (`self.SM_Desk_SM_Drawer`)))
  (:`Triggered`
    (`Widget.RemoveFromParent` (`self.InteractWidget_Ref`))
    (set `self.InitalLocation` _relativelocation)
    (set `self.TargetLocation` (`KismetMathLibrary.MakeVector` (- (.x _relativelocation) 32.0)))
    (bind (_direction _newtrack_0) (`Timeline|OpenDrawer`)
      (:`Update`
        (bind _returnvalue_x (`KismetMathLibrary.BreakVector` (`KismetMathLibrary.VLerp` (`self.InitalLocation`) (`self.TargetLocation`) _newtrack_0)))
        (`SceneComponent.K2_SetRelativeLocation` (`self.SM_Desk_SM_Drawer`) (`KismetMathLibrary.MakeVector` _returnvalue_x) false false)))))

(event `self.Box.OnComponentBeginOverlap`
  (params (OverlappedComponent :type "PrimitiveComponent Object Reference") (OtherActor :type "Actor Object Reference") (OtherComp :type "PrimitiveComponent Object Reference") (OtherBodyIndex :type Integer) (bFromSweep :type Boolean) (SweepResult :type "HitResult Structure (by ref)"))
  (cast `/Game/FirstPerson/Blueprints/BP_FirstPersonCharacter` OtherActor)
  (bind _returnvalue (`|CreateWidget` "/Game/Widgets/W_Interact.W_Interact_C"))
  (bind _output_get (set `self.InteractWidget_Ref` _returnvalue))
  (`UserWidget.AddToViewport` _output_get 0)
  (`self.EnableInput` (`GameplayStatics.GetPlayerController` 0)))

(event `self.Box.OnComponentEndOverlap`
  (params (OverlappedComponent :type "PrimitiveComponent Object Reference") (OtherActor :type "Actor Object Reference") (OtherComp :type "PrimitiveComponent Object Reference") (OtherBodyIndex :type Integer))
  (`WidgetLayoutLibrary.RemoveAllWidgets`)
  (cast `/Game/FirstPerson/Blueprints/BP_FirstPersonCharacter` OtherActor)
  (`self.DisableInput` (`GameplayStatics.GetPlayerController` 0)))

(fn `UserConstructionScript`)