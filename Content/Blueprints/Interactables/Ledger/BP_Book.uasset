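; BP_Book is an interactable ledger that the player can inspect or add a held paper to.
; On BeginPlay it spawns a BP_LedgerCam above itself, pitched downward, and attaches it.
; Interacting while holding a BP_BookPaper destroys that item and, after a short delay, reveals the Page component.
; Otherwise, interacting toggles the view target between player and ledger camera, disabling the player's camera movement during inspection.
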(event `self.ReceiveBeginPlay`
  (bind (_returnvalue_roll _returnvalue_pitch _returnvalue_yaw) (`KismetMathLibrary.BreakRotator` (`self.K2_GetActorRotation`)))
  (bind _returnvalue (`|SpawnActorFromClass` "/Game/Blueprints/Interactables/Ledger/BP_LedgerCam.BP_LedgerCam_C" (`KismetMathLibrary.MakeTransform` (+ (`self.K2_GetActorLocation`) (0.0 0.0 40.0)) (`KismetMathLibrary.MakeRotator` _returnvalue_roll (+ _returnvalue_pitch -90.0) (+ _returnvalue_yaw -90.0))) "Undefined" "MultiplyWithRoot" null null))
  (bind _output_get (set `self.CamRef` _returnvalue))
  (`self.K2_AttachToActor` _output_get self "None" "KeepWorld" "KeepWorld" "KeepWorld" true))

(event `/Game/Blueprints/Interactables/BPI_Interactable.InteractWith`
  (params (PlayerChar :type "/Game/FirstPerson/Blueprints/BP_FirstPersonCharacter Object Reference"))
  (bind _returnvalue (`GameplayStatics.GetPlayerController` 0))
  (bind _playerref (`self.PlayerRef`))
  (bind _output_get (set `self.PlayerRef` PlayerChar))
  (if (`KismetMathLibrary.ClassIsChildOf` (`GameplayStatics.GetObjectClass` (`/Game/FirstPerson/Blueprints/BP_FirstPersonCharacter.HeldItem` _output_get)) "/Game/Blueprints/Interactables/Items/BP_BookPaper.BP_BookPaper_C")
    (`self.K2_DestroyActor` (`/Game/FirstPerson/Blueprints/BP_FirstPersonCharacter.HeldItem` (`self.PlayerRef`)))
    (`KismetSystemLibrary.Delay` 0.2)
    (`SceneComponent.SetVisibility` (`self.Page`) true false)
    (set `/Game/FirstPerson/Blueprints/BP_FirstPersonCharacter.HeldItem` null (`self.PlayerRef`))
    (elif (`self.IsInspecting?`)
      (`PlayerController.SetViewTargetWithBlend` _returnvalue (`self.PlayerRef`) 0.0 "VTBlend_Linear" 0.0 false)
      (set `self.IsInspecting?` false)
      (set `/Game/FirstPerson/Blueprints/BP_FirstPersonCharacter.CameraMove?` true _playerref)
      (else
        (`PlayerController.SetViewTargetWithBlend` _returnvalue (`self.CamRef`) 0.0 "VTBlend_Linear" 0.0 false)
        (set `self.IsInspecting?` true)
        (set `/Game/FirstPerson/Blueprints/BP_FirstPersonCharacter.CameraMove?` false _playerref)))))

(fn `UserConstructionScript`)