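; Work-in-progress hint controller built on the DT_Hints and DT_Audio data tables, mostly unwired.
; The GetHints event looks up the DT_Hints row at RowIndex and only prints debug text.
; BeginPlay, WhatStepWeOn? and the Get Hints function are empty.
; Disconnected nodes sketch an index-checked dialogue lookup and hard-coded per-step hint lookups, mostly gated by IsComplete, plus 2D hint audio playback.
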(event `GetHints`
  ;[1 1 1] GetHints
  (bind _outrownames (`DataTableFunctionLibrary.GetDataTableRowNames` "/Game/Blueprints/Data_Tables/DT_Hints.DT_Hints"))
  (bind _output (`|GetArrayItem` _outrownames (`self.Row Index`)))
  (`|GetDataTableRow` "/Game/Blueprints/Data_Tables/DT_Hints.DT_Hints" _output
    (:`then`
      (`KismetSystemLibrary.PrintString` (`KismetStringLibrary.Conv_NameToString` _output) true true (struct :`R` 0.02423 :`G` 1.0 :`A` 1.0) 10.0 "HintRowFound")
      (for _array_element (`|MakeArray` (`KismetArrayLibrary.Array_Length` _outrownames))
        (`KismetSystemLibrary.PrintString` (`KismetStringLibrary.Conv_IntToString` _array_element))))
    (:`RowNotFound`
      (`KismetSystemLibrary.PrintString` "RowNotFound" true true (struct :`G` 0.66 :`B` 1.0 :`A` 1.0) 10.0 "HintRowNotFound"))))

(event `self.ReceiveBeginPlay`)

(event `WhatStepWeOn?`)

(fn `Get Hints`
  (returns (Dialogue :type Text)))

(fn `UserConstructionScript`)