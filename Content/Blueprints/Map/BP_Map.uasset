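; Map puzzle board that moves the bookshelf once every piece sits in its correct slot.
; Nine colour-named collision zones each pass a slot index on overlap, matched against the BP_MapPieces PuzzleLocation to set or clear that entry in RightPiecePlaced.
; Each begin overlap then rechecks the array and, when all entries are true, calls MoveBookshelf on the BP_Bookshelf found in the level.
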(event `self.DarkBlueCollision.OnComponentBeginOverlap`
  (params (OverlappedComponent :type "PrimitiveComponent Object Reference") (OtherActor :type "Actor Object Reference") (OtherComp :type "PrimitiveComponent Object Reference") (OtherBodyIndex :type Integer) (bFromSweep :type Boolean) (SweepResult :type "HitResult Structure (by ref)"))
  (`self.SetBoolTrue` OtherActor)
  (`self.PuzzleComplete`))

(event `self.DarkBlueCollision.OnComponentEndOverlap`
  (params (OverlappedComponent :type "PrimitiveComponent Object Reference") (OtherActor :type "Actor Object Reference") (OtherComp :type "PrimitiveComponent Object Reference") (OtherBodyIndex :type Integer))
  (`self.SetBoolFalse` OtherActor))

(event `self.DarkPurpleCollision.OnComponentBeginOverlap`
  (params (OverlappedComponent :type "PrimitiveComponent Object Reference") (OtherActor :type "Actor Object Reference") (OtherComp :type "PrimitiveComponent Object Reference") (OtherBodyIndex :type Integer) (bFromSweep :type Boolean) (SweepResult :type "HitResult Structure (by ref)"))
  (`self.SetBoolTrue` OtherActor 1)
  (`self.PuzzleComplete`))

(event `self.DarkPurpleCollision.OnComponentEndOverlap`
  (params (OverlappedComponent :type "PrimitiveComponent Object Reference") (OtherActor :type "Actor Object Reference") (OtherComp :type "PrimitiveComponent Object Reference") (OtherBodyIndex :type Integer))
  (`self.SetBoolFalse` OtherActor 1))

(event `self.GreenCollision.OnComponentBeginOverlap`
  (params (OverlappedComponent :type "PrimitiveComponent Object Reference") (OtherActor :type "Actor Object Reference") (OtherComp :type "PrimitiveComponent Object Reference") (OtherBodyIndex :type Integer) (bFromSweep :type Boolean) (SweepResult :type "HitResult Structure (by ref)"))
  (`self.SetBoolTrue` OtherActor 2)
  (`self.PuzzleComplete`))

(event `self.GreenCollision.OnComponentEndOverlap`
  (params (OverlappedComponent :type "PrimitiveComponent Object Reference") (OtherActor :type "Actor Object Reference") (OtherComp :type "PrimitiveComponent Object Reference") (OtherBodyIndex :type Integer))
  (`self.SetBoolFalse` OtherActor 2))

(event `self.LightBlueCollision.OnComponentBeginOverlap`
  (params (OverlappedComponent :type "PrimitiveComponent Object Reference") (OtherActor :type "Actor Object Reference") (OtherComp :type "PrimitiveComponent Object Reference") (OtherBodyIndex :type Integer) (bFromSweep :type Boolean) (SweepResult :type "HitResult Structure (by ref)"))
  (`self.SetBoolTrue` OtherActor 3)
  (`self.PuzzleComplete`))

(event `self.LightBlueCollision.OnComponentEndOverlap`
  (params (OverlappedComponent :type "PrimitiveComponent Object Reference") (OtherActor :type "Actor Object Reference") (OtherComp :type "PrimitiveComponent Object Reference") (OtherBodyIndex :type Integer))
  (`self.SetBoolFalse` OtherActor 3))

(event `self.LightPurpleCollision.OnComponentBeginOverlap`
  (params (OverlappedComponent :type "PrimitiveComponent Object Reference") (OtherActor :type "Actor Object Reference") (OtherComp :type "PrimitiveComponent Object Reference") (OtherBodyIndex :type Integer) (bFromSweep :type Boolean) (SweepResult :type "HitResult Structure (by ref)"))
  (`self.SetBoolTrue` OtherActor 4)
  (`self.PuzzleComplete`))

(event `self.LightPurpleCollision.OnComponentEndOverlap`
  (params (OverlappedComponent :type "PrimitiveComponent Object Reference") (OtherActor :type "Actor Object Reference") (OtherComp :type "PrimitiveComponent Object Reference") (OtherBodyIndex :type Integer))
  (`self.SetBoolFalse` OtherActor 4))

(event `self.OrangeCollision.OnComponentBeginOverlap`
  (params (OverlappedComponent :type "PrimitiveComponent Object Reference") (OtherActor :type "Actor Object Reference") (OtherComp :type "PrimitiveComponent Object Reference") (OtherBodyIndex :type Integer) (bFromSweep :type Boolean) (SweepResult :type "HitResult Structure (by ref)"))
  (`self.SetBoolTrue` OtherActor 5)
  (`self.PuzzleComplete`))

(event `self.OrangeCollision.OnComponentEndOverlap`
  (params (OverlappedComponent :type "PrimitiveComponent Object Reference") (OtherActor :type "Actor Object Reference") (OtherComp :type "PrimitiveComponent Object Reference") (OtherBodyIndex :type Integer))
  (`self.SetBoolFalse` OtherActor 5))

(event `self.PinkCollision.OnComponentBeginOverlap`
  (params (OverlappedComponent :type "PrimitiveComponent Object Reference") (OtherActor :type "Actor Object Reference") (OtherComp :type "PrimitiveComponent Object Reference") (OtherBodyIndex :type Integer) (bFromSweep :type Boolean) (SweepResult :type "HitResult Structure (by ref)"))
  (`self.SetBoolTrue` OtherActor 6)
  (`self.PuzzleComplete`))

(event `self.PinkCollision.OnComponentEndOverlap`
  (params (OverlappedComponent :type "PrimitiveComponent Object Reference") (OtherActor :type "Actor Object Reference") (OtherComp :type "PrimitiveComponent Object Reference") (OtherBodyIndex :type Integer))
  (`self.SetBoolFalse` OtherActor 6))

(event `self.RedCollision.OnComponentBeginOverlap`
  (params (OverlappedComponent :type "PrimitiveComponent Object Reference") (OtherActor :type "Actor Object Reference") (OtherComp :type "PrimitiveComponent Object Reference") (OtherBodyIndex :type Integer) (bFromSweep :type Boolean) (SweepResult :type "HitResult Structure (by ref)"))
  (`self.SetBoolTrue` OtherActor 7)
  (`self.PuzzleComplete`))

(event `self.RedCollision.OnComponentEndOverlap`
  (params (OverlappedComponent :type "PrimitiveComponent Object Reference") (OtherActor :type "Actor Object Reference") (OtherComp :type "PrimitiveComponent Object Reference") (OtherBodyIndex :type Integer))
  (`self.SetBoolFalse` OtherActor 7))

(event `self.YellowCollision.OnComponentBeginOverlap`
  (params (OverlappedComponent :type "PrimitiveComponent Object Reference") (OtherActor :type "Actor Object Reference") (OtherComp :type "PrimitiveComponent Object Reference") (OtherBodyIndex :type Integer) (bFromSweep :type Boolean) (SweepResult :type "HitResult Structure (by ref)"))
  (`self.SetBoolTrue` OtherActor 8)
  (`self.PuzzleComplete`))

(event `self.YellowCollision.OnComponentEndOverlap`
  (params (OverlappedComponent :type "PrimitiveComponent Object Reference") (OtherActor :type "Actor Object Reference") (OtherComp :type "PrimitiveComponent Object Reference") (OtherBodyIndex :type Integer))
  (`self.SetBoolFalse` OtherActor 8))

(fn `PuzzleComplete`
  (locals (Flag :type Boolean))
  (set `local.Flag` false)
  (for _array_element (`self.RightPiecePlaced`)
    (if (not _array_element)
      (set `local.Flag` true)))
  (if (not (`local.Flag`))
    (`KismetSystemLibrary.PrintString` "Puzzle Completed")
    (bind _returnvalue (`GameplayStatics.GetActorOfClass` "/Game/Blueprints/Bookshelf/BP_Bookshelf.BP_Bookshelf_C"))
    (`/Game/Blueprints/Bookshelf/BP_Bookshelf.MoveBookshelf` _returnvalue)))

(fn `SetBoolFalse`
  (params (Object :type "Object Object Reference") (CorrectLoc :type Integer))
  (bind _asbp_map_pieces (cast `/Game/Blueprints/Map/BP_MapPieces` Object))
  (if (== (`/Game/Blueprints/Map/BP_MapPieces.PuzzleLocation` _asbp_map_pieces) CorrectLoc)
    (`KismetArrayLibrary.Array_Set` (`self.RightPiecePlaced`) CorrectLoc)
    (else
      (`KismetSystemLibrary.PrintString` "Wrong Piece"))))

(fn `SetBoolTrue`
  (params (Object :type "Object Object Reference") (CorrectLoc :type Integer))
  (bind _asbp_map_pieces (cast `/Game/Blueprints/Map/BP_MapPieces` Object))
  (if (== (`/Game/Blueprints/Map/BP_MapPieces.PuzzleLocation` _asbp_map_pieces) CorrectLoc)
    (`KismetArrayLibrary.Array_Set` (`self.RightPiecePlaced`) CorrectLoc true)
    (`KismetSystemLibrary.PrintString` "Correct Piece")))

(fn `UserConstructionScript`)