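; Interactive wardrobe that hides a secret passage, opened by the first-person character in two stages.
; A box overlap shows an interact prompt widget and enables input while the player is inside.
; The first secondary-interact press swings the front door open; once open, another press pushes a button and slides the back panel aside.
; Each stage is a one-shot timeline lerp, and the interaction box is destroyed shortly after the button press.
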(event `self.Box.OnComponentBeginOverlap`
  (params (OverlappedComponent :type "PrimitiveComponent Object Reference") (OtherActor :type "Actor Object Reference") (OtherComp :type "PrimitiveComponent Object Reference") (OtherBodyIndex :type Integer) (bFromSweep :type Boolean) (SweepResult :type "HitResult Structure (by ref)"))
  (cast `/Game/FirstPerson/Blueprints/BP_FirstPersonCharacter` OtherActor)
  (bind _returnvalue (`|CreateWidget` "/Game/Widgets/W_FInteract.W_FInteract_C"))
  (bind _output_get (set `self.Wig_Interact_Ref` _returnvalue))
  (`UserWidget.AddToViewport` _output_get 0)
  (`self.EnableInput` (`GameplayStatics.GetPlayerController` 0)))

(event `self.Box.OnComponentEndOverlap`
  (params (OverlappedComponent :type "PrimitiveComponent Object Reference") (OtherActor :type "Actor Object Reference") (OtherComp :type "PrimitiveComponent Object Reference") (OtherBodyIndex :type Integer))
  (cast `/Game/FirstPerson/Blueprints/BP_FirstPersonCharacter` OtherActor)
  (`Widget.RemoveFromParent` (`self.Wig_Interact_Ref`))
  (`self.DisableInput` (`GameplayStatics.GetPlayerController` 0)))

(event `EnhancedInput|/Game/FirstPerson/Input/Actions/IA_SecondaryInteract`
  (params (ActionValue :type Boolean) (ElapsedSeconds :type "Float (double-precision)") (TriggeredSeconds :type "Float (double-precision)") (InputAction :type "InputAction Object Reference" :default "/Game/FirstPerson/Input/Actions/IA_SecondaryInteract.IA_SecondaryInteract"))
  (:`Triggered`
    (if (`self.DoorOpen`)
      (`self.PushButton`)
      (`self.HiddenDoorOpen`)
      (else
        (`self.OpenDoor`)))))

(event `OpenDoor`
  (bind _relativerotation (`SceneComponent.RelativeRotation` (`self.SM_Wardrobe_FrontDoor`)))
  (`/Engine/EditorBlueprintResources/StandardMacros.DoOnce` false
    (:`Completed`
      (set `self.InitialRotation` _relativerotation)
      (set `self.TargetRotation` (`KismetMathLibrary.MakeRotator` 0.0 0.0 (+ (.yaw _relativerotation) -85.63)))
      (bind (_direction _newtrack_0) (`Timeline|T_OpenDoor` :!via `PlayFromStart`)
        (:`Update`
          (bind (_returnvalue_roll _returnvalue_pitch _returnvalue_yaw) (`KismetMathLibrary.BreakRotator` (`KismetMathLibrary.RLerp` (`self.InitialRotation`) (`self.TargetRotation`) _newtrack_0)))
          (`SceneComponent.K2_SetRelativeRotation` (`self.SM_Wardrobe_FrontDoor`) (`KismetMathLibrary.MakeRotator` 0.0 0.0 _returnvalue_yaw) false false))
        (:`Finished`
          (set `self.DoorOpen` true))))))

(event `PushButton`
  (bind _relativelocation (`SceneComponent.RelativeLocation` (`self.SM_Wardrobe_Button`)))
  (`/Engine/EditorBlueprintResources/StandardMacros.DoOnce` false
    (:`Completed`
      (set `self.InitalButtonLocation` _relativelocation)
      (set `self.TargetButtonLocation` (`KismetMathLibrary.MakeVector` (+ (.x _relativelocation) 0.270534) (.y _relativelocation) (.z _relativelocation)))
      (bind (_direction _newtrack_0) (`Timeline|ButtonPress` :!via `PlayFromStart`)
        (:`Update`
          (`SceneComponent.K2_SetRelativeLocation` (`self.SM_Wardrobe_Button`) (`KismetMathLibrary.VLerp` (`self.InitalButtonLocation`) (`self.TargetButtonLocation`) _newtrack_0) false false))
        (:`Finished`
          (`KismetSystemLibrary.Delay` 2.0)
          (`ActorComponent.K2_DestroyComponent` (`self.Box`)))))))

(event `HiddenDoorOpen`
  (bind _relativelocation (`SceneComponent.RelativeLocation` (`self.SM_Wardrobe_BackDoor`)))
  (`/Engine/EditorBlueprintResources/StandardMacros.DoOnce` false
    (:`Completed`
      (set `self.InitialDoorLocation` _relativelocation)
      (set `self.TargetDoorLocation` (`KismetMathLibrary.MakeVector` (- (.x _relativelocation) 80.0) (.y _relativelocation) (.z _relativelocation)))
      (bind (_direction _newtrack_0) (`Timeline|BackDoorOpen` :!via `PlayFromStart`)
        (:`Update`
          (`SceneComponent.K2_SetRelativeLocation` (`self.SM_Wardrobe_BackDoor`) (`KismetMathLibrary.VLerp` (`self.InitialDoorLocation`) (`self.TargetDoorLocation`) _newtrack_0) false false))))))

(fn `UserConstructionScript`)