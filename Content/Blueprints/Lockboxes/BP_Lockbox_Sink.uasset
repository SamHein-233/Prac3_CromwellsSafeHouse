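; Lockbox actor that the first-person player can open with the secondary interact input when PlayerHasKey is true.
; Box overlap shows an interact widget and enables input; leaving clears all widgets and disables input for that character.
; Interaction runs OpenBox once, which calls LockboxEvent.
; Lockbox_Event removes the prompt and plays a timeline to rotate the lid, though a DoOnce applies only the first update.
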(event `self.ReceiveBeginPlay`
  (`ActorComponent.SetActive` (`self.Box`) false false))

(event `EnhancedInput|/Game/FirstPerson/Input/Actions/IA_SecondaryInteract`
  (params (ActionValue :type Boolean) (ElapsedSeconds :type "Float (double-precision)") (TriggeredSeconds :type "Float (double-precision)") (InputAction :type "InputAction Object Reference" :default "/Game/FirstPerson/Input/Actions/IA_SecondaryInteract.IA_SecondaryInteract"))
  (:`Triggered`
    (if (`self.PlayerHasKey?`)
      (`/Engine/EditorBlueprintResources/StandardMacros.DoOnce` false
        (:`Completed`
          (`self.OpenBox`)
          (`KismetSystemLibrary.PrintString` "Function Called")))
      (else
        (`KismetSystemLibrary.PrintString` "Lock still engaged")))))

(event `self.Box.OnComponentBeginOverlap`
  (params (OverlappedComponent :type "PrimitiveComponent Object Reference") (OtherActor :type "Actor Object Reference") (OtherComp :type "PrimitiveComponent Object Reference") (OtherBodyIndex :type Integer) (bFromSweep :type Boolean) (SweepResult :type "HitResult Structure (by ref)"))
  (cast `/Game/FirstPerson/Blueprints/BP_FirstPersonCharacter` OtherActor)
  (bind _returnvalue (`|CreateWidget` "/Game/Widgets/W_EInteract.W_EInteract_C"))
  (bind _output_get (set `self.InteractWidget` _returnvalue))
  (`UserWidget.AddToViewport` _output_get 0)
  (`self.EnableInput` (`GameplayStatics.GetPlayerController` 0)))

(event `self.Box.OnComponentEndOverlap`
  (params (OverlappedComponent :type "PrimitiveComponent Object Reference") (OtherActor :type "Actor Object Reference") (OtherComp :type "PrimitiveComponent Object Reference") (OtherBodyIndex :type Integer))
  (`WidgetLayoutLibrary.RemoveAllWidgets`)
  (cast `/Game/FirstPerson/Blueprints/BP_FirstPersonCharacter` OtherActor)
  (`self.DisableInput` (`GameplayStatics.GetPlayerController` 0)))

(event `Lockbox_Event`
  (bind _relativerotation (`SceneComponent.RelativeRotation` (`self.SM_LockBox_SM_BoxLid`)))
  (`Widget.RemoveFromParent` (`self.InteractWidget`))
  (bind _output_get (set `self.TargetRelativeRotation` (`KismetMathLibrary.MakeRotator` (+ (.roll _relativerotation) -36.0))))
  (bind (_direction _newtrack_0) (`Timeline|OpenLockBox` :!via `PlayFromStart`)
    (:`Update`
      (`/Engine/EditorBlueprintResources/StandardMacros.DoOnce` false
        (:`Completed`
          (bind _returnvalue_roll (`KismetMathLibrary.BreakRotator` (`KismetMathLibrary.RLerp` _output_get _relativerotation _newtrack_0)))
          (`SceneComponent.K2_SetRelativeRotation` (`self.SM_LockBox_SM_BoxLid`) (`KismetMathLibrary.MakeRotator` _returnvalue_roll) false false))))))

(fn `OpenBox`
  (`self.Lockbox_Event`)
  (`KismetSystemLibrary.PrintString` "Function ran"))

(fn `UserConstructionScript`)