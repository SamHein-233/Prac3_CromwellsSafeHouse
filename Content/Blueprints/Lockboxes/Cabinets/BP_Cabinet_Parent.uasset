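; Parent Blueprint for lockbox cabinets, providing a one-time door opening for a locked cabinet.
; OpenDoor caches the left door's relative rotation, then a timeline lerps its yaw through a 140-degree swing.
; When the timeline finishes, the lock hinge and loop components are destroyed.
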(event `OpenDoor`
  (bind _relativerotation (`SceneComponent.RelativeRotation` (`self.SM_CenterCabinet_LeftDoor`)))
  (`/Engine/EditorBlueprintResources/StandardMacros.DoOnce` false
    (:`Completed`
      (set `self.InitialRotation` _relativerotation)
      (set `self.TargetRotation` (`KismetMathLibrary.MakeRotator` 0.0 0.0 (+ (.yaw _relativerotation) 140.0)))
      (bind (_direction _newtrack_0) (`Timeline|OpenCabinetDoor` :!via `PlayFromStart`)
        (:`Update`
          (bind (_returnvalue_roll _returnvalue_pitch _returnvalue_yaw) (`KismetMathLibrary.BreakRotator` (`KismetMathLibrary.RLerp` (`self.InitialRotation`) (`self.TargetRotation`) _newtrack_0)))
          (`SceneComponent.K2_SetRelativeRotation` (`self.SM_CenterCabinet_LeftDoor`) (`KismetMathLibrary.MakeRotator` 0.0 0.0 _returnvalue_yaw) false false))
        (:`Finished`
          (`ActorComponent.K2_DestroyComponent` (`self.SM_CabinetLock_SM_LockHinge`))
          (`ActorComponent.K2_DestroyComponent` (`self.SM_CabinetLock_SM_LockLoop`)))))))

(fn `UserConstructionScript`)