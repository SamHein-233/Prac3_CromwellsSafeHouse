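; Blacklight lockbox Blueprint that opens on secondary interact once its UnlockBoxBlacklight flag is set, and plays a denied sound otherwise.
; When unlocked, player overlap with the Box trigger shows the interact widget and enables input on the actor.
; A DoOnce guards opening, which calls OpenBox, destroys the trigger after a short delay and updates the row index on the level's BP_HintController.
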(event `self.ReceiveBeginPlay`
  (`parent.ReceiveBeginPlay`)
  (bind _returnvalue (`GameplayStatics.GetActorOfClass` "/Game/Blueprints/BP_HintController.BP_HintController_C"))
  (set `self.Hints` _returnvalue))

(event `EnhancedInput|/Game/FirstPerson/Input/Actions/IA_SecondaryInteract`
  (params (ActionValue :type Boolean) (ElapsedSeconds :type "Float (double-precision)") (TriggeredSeconds :type "Float (double-precision)") (InputAction :type "InputAction Object Reference" :default "/Game/FirstPerson/Input/Actions/IA_SecondaryInteract.IA_SecondaryInteract"))
  (:`Triggered`
    (if (`self.UnlockBox_Blacklight`)
      (`/Engine/EditorBlueprintResources/StandardMacros.DoOnce` false
        (:`Completed`
          (`self.OpenBox`)
          (`GameplayStatics.GetActorOfClass` "/Game/Blueprints/Blacklight/BP_Blacklight.BP_Blacklight_C")
          (`KismetSystemLibrary.Delay` 0.5)
          (`ActorComponent.K2_DestroyComponent` (`self.Box`))
          (set `/Game/Blueprints/BP_HintController.Row Index` 14 (`self.Hints`))))
      (else
        (`GameplayStatics.PlaySound2D` "/Game/Blueprints/Audio/Alert_Sounds/Denied.Denied" 1.0 1.0 0.0 null null)))))

(event `self.Box.OnComponentBeginOverlap`
  (params (OverlappedComponent :type "PrimitiveComponent Object Reference") (OtherActor :type "Actor Object Reference") (OtherComp :type "PrimitiveComponent Object Reference") (OtherBodyIndex :type Integer) (bFromSweep :type Boolean) (SweepResult :type "HitResult Structure (by ref)"))
  (if (`self.UnlockBox_Blacklight`)
    (cast `/Game/FirstPerson/Blueprints/BP_FirstPersonCharacter` OtherActor)
    (`UserWidget.AddToViewport` (`self.Wig_Interact_Ref`) 0)
    (`self.EnableInput` (`GameplayStatics.GetPlayerController` 0))))

(fn `UserConstructionScript`
  (`parent.UserConstructionScript`))