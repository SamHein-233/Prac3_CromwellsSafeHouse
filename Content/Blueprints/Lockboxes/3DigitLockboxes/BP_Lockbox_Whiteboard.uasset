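; Whiteboard lockbox actor, filed with the three-digit lockboxes, that the player can open once its whiteboard lock is unlocked.
; While unlocked, first-person character overlap with the Box trigger shows an interact widget and enables input.
; Secondary interact then calls OpenBox once and destroys the trigger, or plays a denied sound if still locked.
; The unlock flag is only read here, never set.
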(event `EnhancedInput|/Game/FirstPerson/Input/Actions/IA_SecondaryInteract`
  (params (ActionValue :type Boolean) (ElapsedSeconds :type "Float (double-precision)") (TriggeredSeconds :type "Float (double-precision)") (InputAction :type "InputAction Object Reference" :default "/Game/FirstPerson/Input/Actions/IA_SecondaryInteract.IA_SecondaryInteract"))
  (:`Triggered`
    (if (`self.WhiteboardLockUnlocked?`)
      (`/Engine/EditorBlueprintResources/StandardMacros.DoOnce` false
        (:`Completed`
          (`self.OpenBox`)
          (`ActorComponent.K2_DestroyComponent` (`self.Box`))))
      (else
        (`GameplayStatics.PlaySound2D` "/Game/Blueprints/Audio/Alert_Sounds/Denied.Denied" 1.0 1.0 0.0 null null)))))

(event `self.Box.OnComponentBeginOverlap`
  (params (OverlappedComponent :type "PrimitiveComponent Object Reference") (OtherActor :type "Actor Object Reference") (OtherComp :type "PrimitiveComponent Object Reference") (OtherBodyIndex :type Integer) (bFromSweep :type Boolean) (SweepResult :type "HitResult Structure (by ref)"))
  (if (`self.WhiteboardLockUnlocked?`)
    (cast `/Game/FirstPerson/Blueprints/BP_FirstPersonCharacter` OtherActor)
    (`UserWidget.AddToViewport` (`self.Wig_Interact_Ref`) 0)
    (`self.EnableInput` (`GameplayStatics.GetPlayerController` 0))))

(fn `UserConstructionScript`
  (`parent.UserConstructionScript`))