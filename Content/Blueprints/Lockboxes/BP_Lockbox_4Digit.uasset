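; Lockbox actor that the first-person character opens by pressing E; despite the 4-digit name, no code entry is present.
; Overlapping the box collision shows an interact widget and enables input, while ending overlap clears all widgets and disables input.
; E removes the prompt and plays a timeline, but a DoOnce lets only its first update rotate the lid's roll.
; When the timeline finishes, the collision is destroyed.
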(event `self.ReceiveBeginPlay`)

(event `Key|E`
  (params (Key :type "Key Structure"))
  (bind _relativerotation (`SceneComponent.RelativeRotation` (`self.Lid`)))
  (:`Pressed`
    (`Widget.RemoveFromParent` (`self.InteractWidget`))
    (bind _output_get (set `self.TargetRelativeRotation` (`KismetMathLibrary.MakeRotator` (+ (.roll _relativerotation) -36.0))))
    (bind (_direction _newtrack_0) (`Timeline|OpenLockBox` :!via `PlayFromStart`)
      (:`Update`
        (`/Engine/EditorBlueprintResources/StandardMacros.DoOnce` false
          (:`Completed`
            (bind _returnvalue_roll (`KismetMathLibrary.BreakRotator` (`KismetMathLibrary.RLerp` _output_get _relativerotation _newtrack_0)))
            (`SceneComponent.K2_SetRelativeRotation` (`self.Lid`) (`KismetMathLibrary.MakeRotator` _returnvalue_roll) false false))))
      (:`Finished`
        (`ActorComponent.K2_DestroyComponent` (`self.BoxCollision`))))))

(event `self.BoxCollision.OnComponentBeginOverlap`
  (params (OverlappedComponent :type "PrimitiveComponent Object Reference") (OtherActor :type "Actor Object Reference") (OtherComp :type "PrimitiveComponent Object Reference") (OtherBodyIndex :type Integer) (bFromSweep :type Boolean) (SweepResult :type "HitResult Structure (by ref)"))
  (cast `/Game/FirstPerson/Blueprints/BP_FirstPersonCharacter` OtherActor)
  (bind _returnvalue (`|CreateWidget` "/Game/Widgets/W_Interact.W_Interact_C"))
  (bind _output_get (set `self.InteractWidget` _returnvalue))
  (`UserWidget.AddToViewport` _output_get 0)
  (`self.EnableInput` (`GameplayStatics.GetPlayerController` 0)))

(event `self.BoxCollision.OnComponentEndOverlap`
  (params (OverlappedComponent :type "PrimitiveComponent Object Reference") (OtherActor :type "Actor Object Reference") (OtherComp :type "PrimitiveComponent Object Reference") (OtherBodyIndex :type Integer))
  (`WidgetLayoutLibrary.RemoveAllWidgets`)
  (cast `/Game/FirstPerson/Blueprints/BP_FirstPersonCharacter` OtherActor)
  (`self.DisableInput` (`GameplayStatics.GetPlayerController` 0)))

(fn `UserConstructionScript`)