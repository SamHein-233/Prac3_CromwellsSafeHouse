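; BP_3DigitLock_Blacklight is a child Blueprint for the blacklight variant of a three-digit lock, deferring BeginPlay and construction to its parent.
; Its UnlockItem event binds itself to OnUnlocked and prints a debug message.
; A delayed teardown that would destroy the lock and its 3DigitCamRef camera actor is present but disconnected, so it never runs.
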(event `self.ReceiveBeginPlay`
  (`parent.ReceiveBeginPlay`))

(event `UnlockItem`
  (add `self.OnUnlocked` self (delegate `UnlockItem`))
  (`KismetSystemLibrary.PrintString` "Ran after bind event in child"))

(fn `UserConstructionScript`
  (`parent.UserConstructionScript`))