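; Blacklight variant of the three-digit lock, a child Blueprint that opens a code entry view and removes itself once unlocked.
; Secondary interact swaps the interact prompt for the digit widget, sets UI-only input and calls GoToCamera on the BP_3DigitLockCam_Blacklight actor it finds.
; The inherited OnUnlocked event triggers UnlockItem, which destroys the lock and its camera after a short delay, with debug prints.
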(event `self.ReceiveBeginPlay`
  (`parent.ReceiveBeginPlay`)
  (add `self.OnUnlocked` self (delegate `UnlockItem`)))

(event `UnlockItem`
  (bind _cam_ref (`self.Cam_Ref`))
  (`KismetSystemLibrary.PrintString` "Ran after bind event in child")
  (`KismetSystemLibrary.Delay` 0.2)
  (`self.K2_DestroyActor` self)
  (`self.K2_DestroyActor` _cam_ref)
  (`KismetSystemLibrary.PrintText` (`|FormatText` "Deleted: {Self} Deleted: {Cam}" (`KismetSystemLibrary.GetDisplayName` self) (`KismetSystemLibrary.GetDisplayName` _cam_ref))))

(event `EnhancedInput|/Game/FirstPerson/Input/Actions/IA_SecondaryInteract`
  (params (ActionValue :type Boolean) (ElapsedSeconds :type "Float (double-precision)") (TriggeredSeconds :type "Float (double-precision)") (InputAction :type "InputAction Object Reference" :default "/Game/FirstPerson/Input/Actions/IA_SecondaryInteract.IA_SecondaryInteract"))
  (:`Triggered`
    (`Widget.RemoveFromParent` (`self.Wig_Interact_Ref`))
    (bind _asbp_first_person_character (cast `/Game/FirstPerson/Blueprints/BP_FirstPersonCharacter` (`GameplayStatics.GetPlayerPawn` 0)))
    (bind _returnvalue (`UserWidget.AddToPlayerScreen` (`self.DigitWidget_Ref`) 0))
    (`WidgetBlueprintLibrary.SetInputMode_UIOnlyEx` (`Pawn.GetLocalViewingPlayerController` _asbp_first_person_character) null "DoNotLock" _returnvalue)
    (bind _returnvalue_2 (`GameplayStatics.GetActorOfClass` "/Game/Blueprints/Digitlocks/3DigitCameras/BP_3DigitLockCam_Blacklight.BP_3DigitLockCam_Blacklight_C"))
    (bind _output_get (set `self.Cam_Ref` _returnvalue_2))
    (`/Game/Blueprints/Digitlocks/3DigitCameras/BP_3DigitLockCam.GoToCamera` _output_get)))

(fn `UserConstructionScript`
  (`parent.UserConstructionScript`))