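; Child digit padlock for a riddle puzzle that opens the riddle cabinet when unlocked.
; On BeginPlay it finds the hint controller and cabinet, then binds the inherited unlock event.
; Secondary interact shows the digit widget in UI-only input and blends the view to the lock, while box overlap caches the lock camera.
; Unlocking briefly waits, opens the cabinet door, destroys the lock, sets the hint row and plays a sound.
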(event `self.ReceiveBeginPlay`
  (`parent.ReceiveBeginPlay`)
  (bind _returnvalue (`GameplayStatics.GetActorOfClass` "/Game/Blueprints/BP_HintController.BP_HintController_C"))
  (set `self.Hints` _returnvalue)
  (bind _returnvalue_2 (`GameplayStatics.GetActorOfClass` "/Game/Blueprints/Lockboxes/Cabinets/BP_Cabinet_Riddle.BP_Cabinet_Riddle_C"))
  (set `self.Cabinet_Ref` _returnvalue_2)
  (add `self.OnUnlocked` self (delegate `UnlockItem`)))

(event `UnlockItem`
  (`KismetSystemLibrary.Delay` 0.2)
  (`/Game/Blueprints/Lockboxes/Cabinets/BP_Cabinet_Parent.OpenDoor` (`self.Cabinet_Ref`))
  (`self.K2_DestroyActor` self)
  (set `/Game/Blueprints/BP_HintController.Row Index` 10 (`self.Hints`))
  (`GameplayStatics.PlaySound2D` "/Game/Blueprints/Audio/Dialogue/CromwellDialogue/MS_5_1.MS_5_1" 1.0 1.0 0.0 null null))

(event `EnhancedInput|/Game/FirstPerson/Input/Actions/IA_SecondaryInteract`
  (params (ActionValue :type Boolean) (ElapsedSeconds :type "Float (double-precision)") (TriggeredSeconds :type "Float (double-precision)") (InputAction :type "InputAction Object Reference" :default "/Game/FirstPerson/Input/Actions/IA_SecondaryInteract.IA_SecondaryInteract"))
  (bind _digitwidget_ref (`self.DigitWidget_Ref`))
  (:`Started`
    (`Widget.RemoveFromParent` (`self.Wig_Interact_Ref`))
    (bind _asbp_first_person_character (cast `/Game/FirstPerson/Blueprints/BP_FirstPersonCharacter` (`GameplayStatics.GetPlayerPawn` 0)))
    (set `/Game/Widgets/W_3DigitLock.PadLockRef` self _digitwidget_ref)
    (bind _returnvalue (`UserWidget.AddToPlayerScreen` _digitwidget_ref 0))
    (`WidgetBlueprintLibrary.SetInputMode_UIOnlyEx` (`Pawn.GetLocalViewingPlayerController` _asbp_first_person_character) null "DoNotLock" _returnvalue)
    (`PlayerController.SetViewTargetWithBlend` (`GameplayStatics.GetPlayerController` 0) self (`self.BlendTime`) "VTBlend_Linear" 0.0 false)))

(event `self.Box.OnComponentBeginOverlap`
  (params (OverlappedComponent :type "PrimitiveComponent Object Reference") (OtherActor :type "Actor Object Reference") (OtherComp :type "PrimitiveComponent Object Reference") (OtherBodyIndex :type Integer) (bFromSweep :type Boolean) (SweepResult :type "HitResult Structure (by ref)"))
  (bind _asbp_3digit_lock_cam (cast `/Game/Blueprints/Digitlocks/3DigitCameras/BP_3DigitLockCam` OtherActor))
  (set `self.3DigitCam_Ref` _asbp_3digit_lock_cam))

(fn `UserConstructionScript`
  (`parent.UserConstructionScript`))