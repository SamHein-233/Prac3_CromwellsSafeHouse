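; Wardrobe variant of a four-digit padlock, a child Blueprint that unlocks the wardrobe door when solved.
; Secondary interact swaps the interact prompt for the digit widget, sets UI-only input and blends the view to the lock.
; The inherited OnUnlocked event sets the unlocked flag on the BP_Wardrobe found at BeginPlay.
; It then destroys the lock after a short delay and plays an alert, with a second delayed sound sequenced after the destroy.
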(event `self.ReceiveBeginPlay`
  (`parent.ReceiveBeginPlay`)
  (add `self.OnUnlocked` self (delegate `UnlockItem`))
  (bind _returnvalue (`GameplayStatics.GetActorOfClass` "/Game/Blueprints/Wardrobe/BP_Wardrobe.BP_Wardrobe_C"))
  (set `self.BPWardrobe_Ref` _returnvalue))

(event `UnlockItem`
  (`KismetSystemLibrary.PrintString` "Ran after bind event in child")
  (set `/Game/Blueprints/Wardrobe/BP_Wardrobe.WardrobeDoorLockUnlocked?` true (`self.BPWardrobe_Ref`))
  (`KismetSystemLibrary.Delay` 0.2)
  (`self.K2_DestroyActor` self)
  (`GameplayStatics.PlaySound2D` "/Game/Blueprints/Audio/Alert_Sounds/MS_Alert.MS_Alert" 1.0 1.0 0.0 null null)
  (`KismetSystemLibrary.Delay` 0.8)
  (`GameplayStatics.PlaySound2D` "/Game/Blueprints/Audio/Dialogue/CromwellDialogue/Puzzle_6_1.Puzzle_6_1" 1.0 1.0 0.0 null null))

(event `EnhancedInput|/Game/FirstPerson/Input/Actions/IA_SecondaryInteract`
  (params (ActionValue :type Boolean) (ElapsedSeconds :type "Float (double-precision)") (TriggeredSeconds :type "Float (double-precision)") (InputAction :type "InputAction Object Reference" :default "/Game/FirstPerson/Input/Actions/IA_SecondaryInteract.IA_SecondaryInteract"))
  (bind _digitwidget_ref (`self.DigitWidget_Ref`))
  (:`Triggered`
    (`Widget.RemoveFromParent` (`self.Wig_Interact_Ref`))
    (bind _asbp_first_person_character (cast `/Game/FirstPerson/Blueprints/BP_FirstPersonCharacter` (`GameplayStatics.GetPlayerPawn` 0)))
    (set `/Game/Widgets/W_4DigitLock.PadLockRef` self _digitwidget_ref)
    (bind _returnvalue (`UserWidget.AddToPlayerScreen` _digitwidget_ref 0))
    (`WidgetBlueprintLibrary.SetInputMode_UIOnlyEx` (`Pawn.GetLocalViewingPlayerController` _asbp_first_person_character) null "DoNotLock" _returnvalue)
    (`PlayerController.SetViewTargetWithBlend` (`GameplayStatics.GetPlayerController` 0) self (`self.BlendTime`) "VTBlend_Linear" 0.0 false)))

(fn `UserConstructionScript`
  (`parent.UserConstructionScript`))