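; Child four-digit padlock Blueprint that guards the whiteboard lockbox.
; It binds the parent's OnUnlocked event to flag the lockbox as unlocked, then destroys itself after a short delay, with debug prints.
; Secondary interact removes the interact widget, shows the digit widget with this lock as its padlock reference, switches to UI-only input and blends the view to the lock.
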(event `self.ReceiveBeginPlay`
  (`parent.ReceiveBeginPlay`)
  (add `self.OnUnlocked` self (delegate `UnlockItem`)))

(event `UnlockItem`
  (`KismetSystemLibrary.PrintString` "Ran after bind event in child")
  (set `/Game/Blueprints/Lockboxes/3DigitLockboxes/BP_Lockbox_Whiteboard.WhiteboardLockUnlocked?` true (`self.WhiteboardLockbox`))
  (`KismetSystemLibrary.Delay` 0.2)
  (`self.K2_DestroyActor` self)
  (`KismetSystemLibrary.PrintText` (`|FormatText` "Deleted: {Self} Deleted: {Cam}" (`KismetSystemLibrary.GetDisplayName` self) _))
  (set `self.WhiteboardLockboxUnlocked?` true))

(event `EnhancedInput|/Game/FirstPerson/Input/Actions/IA_SecondaryInteract`
  (params (ActionValue :type Boolean) (ElapsedSeconds :type "Float (double-precision)") (TriggeredSeconds :type "Float (double-precision)") (InputAction :type "InputAction Object Reference" :default "/Game/FirstPerson/Input/Actions/IA_SecondaryInteract.IA_SecondaryInteract"))
  (bind _digitwidget_ref (`self.DigitWidget_Ref`))
  (:`Triggered`
    (`Widget.RemoveFromParent` (`self.Wig_Interact_Ref`))
    (bind _asbp_first_person_character (cast `/Game/FirstPerson/Blueprints/BP_FirstPersonCharacter` (`GameplayStatics.GetPlayerPawn` 0)))
    (set `/Game/Widgets/W_4DigitLock.PadLockRef` self _digitwidget_ref)
    (bind _returnvalue (`UserWidget.AddToPlayerScreen` _digitwidget_ref 0))
    (`WidgetBlueprintLibrary.SetInputMode_UIOnlyEx` (`Pawn.GetLocalViewingPlayerController` _asbp_first_person_character) null "DoNotLock" _returnvalue)
    (`PlayerController.SetViewTargetWithBlend` (`GameplayStatics.GetPlayerController` 0) self (`self.BlendTime`) "VTBlend_Linear" 0.0 false)))

(fn `UserConstructionScript`
  (`parent.UserConstructionScript`))