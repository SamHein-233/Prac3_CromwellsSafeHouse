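; Three-digit lock Blueprint for a lockbox, which handles what happens when the lock is unlocked.
; UnlockItem, tied to the OnUnlocked event, finds the BP_LockboxMesh_3Digit actor in the level and spawns an actor at its transform.
; After short delays it destroys that mesh actor, prints an unlock message, then destroys itself and the lock's camera actor.
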(event `self.ReceiveBeginPlay`
  (`parent.ReceiveBeginPlay`))

(event `UnlockItem`
  (add `self.OnUnlocked` (delegate `UnlockItem`))
  (bind _returnvalue (`GameplayStatics.GetActorOfClass` "/Game/Blueprints/Lockboxes/BP_LockboxMesh_3Digit.BP_LockboxMesh_3Digit_C"))
  (`|SpawnActorFromClass` "/Game/Blueprints/Lockboxes/BP_Lockbox_3Digit.BP_Lockbox_3Digit_C" (`self.GetTransform` _returnvalue) "Undefined" "MultiplyWithRoot" null null)
  (`KismetSystemLibrary.Delay` 0.2)
  (`self.K2_DestroyActor` _returnvalue)
  (`KismetSystemLibrary.PrintString` "Lock is unlocked!" true true (struct :`G` 1.0 :`B` 0.051351 :`A` 1.0))
  (`KismetSystemLibrary.Delay` 0.2)
  (`self.K2_DestroyActor`)
  (`self.K2_DestroyActor` (`self.3DigitCam_Ref`)))

(fn `UserConstructionScript`
  (`parent.UserConstructionScript`))