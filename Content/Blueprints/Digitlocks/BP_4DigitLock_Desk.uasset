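; Four-digit combination lock that removes the desk latch and destroys itself and its camera when solved.
; Overlapping its box enables interaction, which opens the lock widget in UI-only input and switches to BP_4DigitLockCam.
; Rotate events step the selected dial's stored digit with wraparound and animate 36-degree turns via DoOnce-gated timelines, though RotateLeft increments dial 4.
; CheckCombination compares all four digits to CorrectCombination, restoring player camera and input on success.
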(event `RotateRight`
  (bind _selecteddigitrow (`self.SelectedDigitRow`))
  (bind _relativerotation (`SceneComponent.RelativeRotation` _selecteddigitrow))
  (`/Engine/EditorBlueprintResources/StandardMacros.DoOnce` false :!label _label
    (:`Completed`
      (bind _dialscombination (`self.SelectedRow` _selecteddigitrow))
      (switch `int` _dialscombination
        (:`0`
          (bind _newint (`self.IncAndMod` (`self.Dial1StoreNum`)))
          (set `self.Dial1StoreNum` _newint))
        (:`1`
          (bind _newint_2 (`self.IncAndMod` (`self.Dial2StoreNum`)))
          (set `self.Dial2StoreNum` _newint_2))
        (:`2`
          (bind _newint_3 (`self.IncAndMod` (`self.Dial3StoreNum`)))
          (set `self.Dial3StoreNum` _newint_3))
        (:`3`
          (bind _newint_4 (`self.IncAndMod` (`self.Dial4StoreNum`)))
          (set `self.Dial4StoreNum` _newint_4)))
      (set `self.InitialRotation` _relativerotation)
      (set `self.TargetRelativeRotation` (`KismetMathLibrary.MakeRotator` 0.0 0.0 (+ (.yaw _relativerotation) 36.0)))
      (bind (_direction _newtrack_0) (`Timeline|RotateDigitRight` :!via `PlayFromStart`)
        (:`Update`
          (bind (_returnvalue_roll _returnvalue_pitch _returnvalue_yaw) (`KismetMathLibrary.BreakRotator` (`KismetMathLibrary.RLerp` (`self.InitialRotation`) (`self.TargetRelativeRotation`) _newtrack_0)))
          (`SceneComponent.K2_SetRelativeRotation` _selecteddigitrow (`KismetMathLibrary.MakeRotator` 0.0 0.0 _returnvalue_yaw) false false))
        (:`Finished`
          (`KismetSystemLibrary.PrintText` (`|FormatText` "1: {int1}   2: {int2}    3: {int3}" (`self.Dial1StoreNum`) (`self.Dial2StoreNum`) (`self.Dial3StoreNum`)) true true (struct :`G` 0.66 :`B` 1.0 :`A` 1.0) 5.0)
          (goto _label :!via `Reset`))))))

(event `self.ReceiveBeginPlay`
  (bind _sm_dial1 (`self.SM_Dial1`))
  (bind _returnvalue (`|CreateWidget` "/Game/Widgets/W_4DigitLock.W_4DigitLock_C"))
  (set `self.DigitWidget_Ref` _returnvalue)
  (`self.SelectedRow` _sm_dial1)
  (set `self.SelectedDigitRow` _sm_dial1))

(event `self.Box.OnComponentBeginOverlap`
  (params (OverlappedComponent :type "PrimitiveComponent Object Reference") (OtherActor :type "Actor Object Reference") (OtherComp :type "PrimitiveComponent Object Reference") (OtherBodyIndex :type Integer) (bFromSweep :type Boolean) (SweepResult :type "HitResult Structure (by ref)"))
  (bind _asbp_first_person_character (cast `/Game/FirstPerson/Blueprints/BP_FirstPersonCharacter` OtherActor))
  (bind _returnvalue (`|CreateWidget` "/Game/Widgets/W_Interact.W_Interact_C"))
  (bind _output_get (set `self.InteractWidget_Ref` _returnvalue))
  (`UserWidget.AddToViewport` _output_get 0)
  (`self.EnableInput` (`GameplayStatics.GetPlayerController` 0)))

(event `EnhancedInput|/Game/FirstPerson/Input/Actions/IA_Interact`
  (params (ActionValue :type Boolean) (ElapsedSeconds :type "Float (double-precision)") (TriggeredSeconds :type "Float (double-precision)") (InputAction :type "InputAction Object Reference" :default "/Game/FirstPerson/Input/Actions/IA_Interact.IA_Interact"))
  (:`Triggered`
    (`Widget.RemoveFromParent` (`self.InteractWidget_Ref`))
    (bind _returnvalue (`UserWidget.AddToPlayerScreen` (`self.DigitWidget_Ref`) 0))
    (`WidgetBlueprintLibrary.SetInputMode_UIOnlyEx` (`Pawn.GetLocalViewingPlayerController` (stale `self.Box.OnComponentBeginOverlap` _asbp_first_person_character)) null "DoNotLock" _returnvalue)
    (bind _returnvalue_2 (`GameplayStatics.GetActorOfClass` "/Game/Blueprints/Digitlocks/BP_4DigitLockCam.BP_4DigitLockCam_C"))
    (set `self.4DigitCam_Ref` _returnvalue_2)
    (`/Game/Blueprints/Digitlocks/BP_4DigitLockCam.GoToCamera` _returnvalue_2)))

(event `self.Box.OnComponentEndOverlap`
  (params (OverlappedComponent :type "PrimitiveComponent Object Reference") (OtherActor :type "Actor Object Reference") (OtherComp :type "PrimitiveComponent Object Reference") (OtherBodyIndex :type Integer))
  (`WidgetLayoutLibrary.RemoveAllWidgets`)
  (cast `/Game/FirstPerson/Blueprints/BP_FirstPersonCharacter` OtherActor)
  (`self.DisableInput` (`GameplayStatics.GetPlayerController` 0)))

(event `RotateLeft`
  (bind _selecteddigitrow (`self.SelectedDigitRow`))
  (bind _relativerotation (`SceneComponent.RelativeRotation` _selecteddigitrow))
  (`/Engine/EditorBlueprintResources/StandardMacros.DoOnce` false :!label _label_2
    (:`Completed`
      (bind _dialscombination (`self.SelectedRow` _selecteddigitrow))
      (switch `int` _dialscombination
        (:`0`
          (bind _newint (`self.DecAndCheck` (`self.Dial1StoreNum`)))
          (set `self.Dial1StoreNum` _newint))
        (:`1`
          (bind _newint_2 (`self.DecAndCheck` (`self.Dial2StoreNum`)))
          (set `self.Dial2StoreNum` _newint_2))
        (:`2`
          (bind _newint_3 (`self.DecAndCheck` (`self.Dial3StoreNum`)))
          (set `self.Dial3StoreNum` _newint_3))
        (:`3`
          (bind _newint_4 (`self.IncAndMod` (`self.Dial4StoreNum`)))
          (set `self.Dial4StoreNum` _newint_4)))
      (set `self.InitialRotation` _relativerotation)
      (set `self.TargetRelativeRotation` (`KismetMathLibrary.MakeRotator` 0.0 0.0 (+ (.yaw _relativerotation) -36.0)))
      (bind (_direction _newtrack_0) (`Timeline|Timeline` :!via `PlayFromStart`)
        (:`Update`
          (bind (_returnvalue_roll _returnvalue_pitch _returnvalue_yaw) (`KismetMathLibrary.BreakRotator` (`KismetMathLibrary.RLerp` (`self.InitialRotation`) (`self.TargetRelativeRotation`) _newtrack_0)))
          (`SceneComponent.K2_SetRelativeRotation` _selecteddigitrow (`KismetMathLibrary.MakeRotator` 0.0 0.0 _returnvalue_yaw) false false))
        (:`Finished`
          (`KismetSystemLibrary.PrintText` (`|FormatText` "1: {int1}   2: {int2}    3: {int3}" (`self.Dial1StoreNum`) (`self.Dial2StoreNum`) (`self.Dial3StoreNum`)) true true (struct :`G` 0.66 :`B` 1.0 :`A` 1.0) 5.0)
          (goto _label_2 :!via `Reset`))))))

(event `CheckCombination`
  (bind _returnvalue (`GameplayStatics.GetPlayerController` 0))
  (bind _correctcombination (`self.CorrectCombination`))
  (if (and (== (`self.Dial1StoreNum`) (`|GetArrayItem` _correctcombination)) (== (`|GetArrayItem` _correctcombination 1) (`self.Dial2StoreNum`)) (== (`|GetArrayItem` _correctcombination 2) (`self.Dial3StoreNum`)) (== (`|GetArrayItem` _correctcombination 3) (`self.Dial4StoreNum`)))
    (`/Game/Blueprints/Digitlocks/BP_4DigitLockCam.GoToPlayer` (`self.4DigitCam_Ref`) (`GameplayStatics.GetPlayerCharacter` 0))
    (`WidgetBlueprintLibrary.SetInputMode_GameOnly` _returnvalue)
    (set `PlayerController.bShowMouseCursor` false _returnvalue)
    (`Widget.RemoveFromParent` (`self.DigitWidget_Ref`))
    (bind _returnvalue_2 (`GameplayStatics.GetActorOfClass` "/Game/Blueprints/Interactables/Desk/BP_Desk.BP_Desk_C"))
    (`KismetSystemLibrary.Delay` 0.2)
    (`ActorComponent.K2_DestroyComponent` (`/Game/Blueprints/Interactables/Desk/BP_Desk.SM_Desk_SM_Latch` _returnvalue_2))
    (`KismetSystemLibrary.PrintString` "Lock is unlocked!" true true (struct :`G` 1.0 :`B` 0.051351 :`A` 1.0))
    (`KismetSystemLibrary.Delay` 0.2)
    (`self.K2_DestroyActor`)
    (`self.K2_DestroyActor` (`self.4DigitCam_Ref`))
    (else
      (`KismetSystemLibrary.PrintString` "Incorrect Combination :(" true true (struct :`R` 1.0 :`B` 0.012891 :`A` 1.0)))))

(fn `DecAndCheck`
  (params (CurInt :type Integer))
  (returns (NewInt :type Integer))
  (bind _result (`/Engine/EditorBlueprintResources/StandardMacros.DecrementInt` CurInt)
    (:`  `
      (if (== _result -1)
        (return 9)
        (else
          (return _result))))))

(fn `IncAndMod`
  (params (CurInt :type Integer))
  (returns (NewInt :type Integer))
  (bind _result (`/Engine/EditorBlueprintResources/StandardMacros.IncrementInt` CurInt)
    (:`  `
      (return (mod _result 10)))))

(fn `SelectedRow`
  (params (DialMesh :type "StaticMeshComponent Object Reference"))
  (returns (DialsCombination :type Integer))
  (bind _output_get (set `self.SelectedDigitRow` DialMesh))
  (if (== _output_get (`self.SM_Dial1`))
    (return 0)
    (elif (== _output_get (`self.SM_Dial2`))
      (return 1)
      (elif (== _output_get (`self.SM_Dial3`))
        (return 2)
        (elif (== _output_get (`self.SM_Dial4`))
          (return 3)
          (else
            (return -1)))))))

(fn `UserConstructionScript`)