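; BP_Blacklight is a blacklight actor that feeds its position to materials, apparently to drive blacklight visibility effects.
; Each Tick writes the SpotLight's world location, shifted 400 units along negative world X, to the BlacklightLocation vector in MPC_BlacklightVisbility.
; The offset is fixed in world space and ignores the light's rotation.
; Logic to switch the light off exists but is unconnected.
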(event `self.ReceiveBeginPlay`)

(event `self.ReceiveTick`
  (params (DeltaSeconds :type "Float (single-precision)"))
  (`KismetMaterialLibrary.SetVectorParameterValue` "/Game/Materials/Decals/MPC_BlacklightVisbility.MPC_BlacklightVisbility" "BlacklightLocation" (`KismetMathLibrary.Conv_VectorToLinearColor` (- (`SceneComponent.K2_GetComponentLocation` (`self.SpotLight`)) (400.0 0.0 0.0)))))

(fn `UserConstructionScript`
  (`parent.UserConstructionScript`))